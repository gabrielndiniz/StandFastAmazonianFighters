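; Sublevel loader Blueprint that brings in a map's geometry, audio and lighting streaming levels on BeginPlay.
; It sets the loaded and visible flags on each streaming level directly, printing an error for any it cannot find.
; LoadGeoLevel acts as a swap: it unloads the stored geometry level, stores the new name, then shows that level if hidden or forced.
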(event EventBeginPlay
  (bind _audiolevel (Variables|Default|GetAudioLevel))
  (bind _lightninglevel (Variables|Default|GetLightningLevel))
  (bind _returnvalue (Utilities|String|StringToName _lightninglevel))
  (bind _returnvalue_2 (Utilities|String|StringToName _audiolevel))
  (bind _returnvalue_3 (Class|GameplayStatics|GetStreamingLevel _returnvalue))
  (bind _returnvalue_4 (Class|GameplayStatics|GetStreamingLevel _returnvalue_2))
  (CallFunction|LoadGeoLevel (Variables|Default|GetGeoLevel) false)
  (Utilities|FlowControl|Sequence
    (:then_0
      (Utilities|IsValid _returnvalue_4
        (:Is%20Valid
          (Variables|/Script/Engine.LevelStreaming|SetbShouldBeLoaded _returnvalue_4 true)
          (Variables|/Script/Engine.LevelStreaming|SetbShouldBeVisible _returnvalue_4 true))
        (:Is%20Not%20Valid
          (Development|PrintString "Error @7j$: Audio Level Not Found: "))))
    (:then_1
      (Utilities|IsValid _returnvalue_3
        (:Is%20Valid
          (Variables|/Script/Engine.LevelStreaming|SetbShouldBeLoaded _returnvalue_3 true)
          (Variables|/Script/Engine.LevelStreaming|SetbShouldBeVisible _returnvalue_3 true))
        (:Is%20Not%20Valid
          (Development|PrintString "Error @7j$: Light Level Not Found: "))))))

(fn ConstructionScript)

(fn LoadGeoLevel
  (params (Level :type String) (ForceLoad :type Boolean))
  (Utilities|FlowControl|Sequence
    (:then_0
      (Utilities|IsValid (Class|GameplayStatics|GetStreamingLevel (Utilities|String|StringToName (Variables|Default|GetStandardGeoLevel)))
        (:Is%20Valid
          (Variables|/Script/Engine.LevelStreaming|SetbShouldBeLoaded (Class|GameplayStatics|GetStreamingLevel (Utilities|String|StringToName (Variables|Default|GetStandardGeoLevel))) false)
          (Variables|/Script/Engine.LevelStreaming|SetbShouldBeVisible (Class|GameplayStatics|GetStreamingLevel (Utilities|String|StringToName (Variables|Default|GetStandardGeoLevel))) false))))
    (:then_1
      (bind _output_get (Variables|Default|SetStandardGeoLevel Level))
      (Utilities|IsValid (Class|GameplayStatics|GetStreamingLevel (Utilities|String|StringToName _output_get))
        (:Is%20Valid
          (if (or (not (Variables|/Script/Engine.LevelStreaming|GetbShouldBeVisible (Class|GameplayStatics|GetStreamingLevel (Utilities|String|StringToName _output_get)))) ForceLoad)
            (Variables|/Script/Engine.LevelStreaming|SetbShouldBeLoaded (Class|GameplayStatics|GetStreamingLevel (Utilities|String|StringToName _output_get)) true)
            (Variables|/Script/Engine.LevelStreaming|SetbShouldBeVisible (Class|GameplayStatics|GetStreamingLevel (Utilities|String|StringToName _output_get)) true)))
        (:Is%20Not%20Valid
          (Development|PrintString (Utilities|String|Append "Error @7j$: Load Geo Level Not Found: " _output_get)))))))