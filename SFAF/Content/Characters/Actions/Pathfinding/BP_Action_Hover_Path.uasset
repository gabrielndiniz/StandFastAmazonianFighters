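; BP_Action_Hover_Path is a grid action that previews the path from a combatant's tile to a target position.
; ExecuteAction runs the parent action, casts the first tile's occupying unit to BP_Combatant_Base, and passes it with both positions to GenerateReachable.
; GenerateReachable clears the old preview, queries the FindPath object, and adds an instanced static mesh slightly above tile height for each path step.
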(fn ConstructionScript
  (|CallParentFunction))

(fn GenerateReachable
  (params (Unit :type BP%20Combatant%20Base%20Object%20Reference) (Position1 :type Int%20Point%20Structure) (Position2 :type Int%20Point%20Structure))
  (bind _grid (Variables|Default|GetGrid))
  (bind _tiledata (Default|GetTileData _grid))
  (bind (_x _y _z) (Math|Vector|BreakVector (.worldlocation _tiledata)))
  (if (!= Unit (Variables|Default|GetCurrentUnit))
    (Variables|Default|SetCurrentUnit Unit))
  (CallFunction|ClearPath)
  (Utilities|IsValid (Variables|Default|GetCurrentUnit)
    (:Is%20Valid
      (bind (_path _bfoundpath) (Default|FindPath (Variables|Default|GetFindPath) Position1 Position2 false false false))
      (if _bfoundpath
        (for _array_element _path
          (Components|InstancedStaticMesh|AddInstance (Variables|Default|GetInstancedStaticMeshPath) (Math|Transform|MakeTransform (Math|Vector|MakeVector _x _y (+ _z 5.0)) "0, 0, 0" "1.000000,1.000000,1.000000") true))))))

(fn SetFindPathtoTarget
  (params (FindPath :type BP%20Action%20Find%20Path%20to%20Target%20Object%20Reference))
  (Variables|Default|SetFindPath FindPath))

(fn ExecuteAction
  (params (Position%201 :type Int%20Point%20Structure) (bHitResult :type Boolean) (Position%202 :type Int%20Point%20Structure))
  (bind (_success _tiledata1 _tiledata2) (|CallParentFunction Position%201 bHitResult Position%202))
  (bind _asbp_combatant_base (Utilities|Casting|CastToBP_Combatant_Base (.occupyingunit (.Occupancy (Utilities|Struct|BreakGridTileStaticData _tiledata1)))))
  (CallFunction|GenerateReachable _asbp_combatant_base Position%201 Position%202)
  (return _success _tiledata1 _tiledata2))

(fn ClearPath
  (Components|InstancedStaticMesh|ClearInstances (Variables|Default|GetInstancedStaticMeshPath)))