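; Grid action that marks and optionally displays the valid pathfinding neighbors of the targeted tile.
; When the position changes, it clears the old Neighbor states, rebuilds the list, tags those tiles on the Grid and can place instanced meshes on them.
; It checks six hex-style candidates, offset by X parity, for walkability, occupancy and movement cost, with toggles for flying units and ignoring units.
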(event EventBeginPlay
  (|CallParentFunction) ; This node is disabled and will not be called.\nDrag off pins to build functionality.
)

(event Collision|EventActorBeginOverlap
  (params (OtherActor :type Actor%20Object%20Reference))
  (|CallParentFunction OtherActor) ; This node is disabled and will not be called.\nDrag off pins to build functionality.
)

(event EventTick
  (params (DeltaSeconds :type Float%20%28single-precision%29))
  (|CallParentFunction DeltaSeconds) ; This node is disabled and will not be called.\nDrag off pins to build functionality.
)

(fn ConstructionScript
  (|CallParentFunction))

(fn ExecuteAction
  (params (Position%201 :type Int%20Point%20Structure) (bHitResult :type Boolean) (Position%202 :type Int%20Point%20Structure))
  (bind (_success _tiledata1 _tiledata2) (|CallParentFunction Position%201 bHitResult Position%202))
  (if (!= Position%201 (Variables|Default|GetCurrentPositon%201))
    (CallFunction|ClearTiles)
    (if bHitResult
      (bind _output_get (Variables|Default|SetCurrentPositon%201 Position%201))
      (bind _neighborpositions (CallFunction|GetValidTileNeighbors _output_get))
      (bind _output_get_2 (Variables|Default|SetValidNeighborPositions _neighborpositions))
      (for _array_element _output_get_2
        (Default|AddStateTile (Variables|Default|GetGrid) (.position _array_element) "Neighbor")
        (CallFunction|ShowNeighbors)
        (return _success _tiledata1 _tiledata2))
      (else
        (Variables|Default|SetCurrentPositon%201 (Utilities|Struct|MakeIntPoint 9999 9999))))
    (else
      (return _success _tiledata1 _tiledata2))))

(fn SetShowNeighbors
  (params (bShowNeighbors :type Boolean))
  (Variables|Default|SetbShowNeighbors bShowNeighbors))

(fn ShowNeighbors
  (Components|InstancedStaticMesh|ClearInstances (Variables|Default|GetInstancedStaticMesh))
  (if (Variables|Default|GetbShowNeighbors)
    (for _array_element (Variables|Default|GetValidNeighborPositions)
      (Components|InstancedStaticMesh|AddInstance (Variables|Default|GetInstancedStaticMesh) (Math|Transform|MakeTransform (.worldlocation (.TileData (Default|GetTileData (Variables|Default|GetGrid) (.position _array_element)))) "0, 0, 0" "1.000000,1.000000,1.000000") true))))

(fn GetValidTileNeighbors
  (params (Position :type Int%20Point%20Structure))
  (LocalVariables|SetXValue (.x Position))
  (LocalVariables|SetYValue (.y Position))
  (for _index (range 0 1)
    (bind _output_get (LocalVariables|SetAddPosition (Utilities|Struct|MakeIntPoint (+ (* _index 4) -2 (LocalVariables|GetXValue)) (LocalVariables|GetYValue))))
    (bind (_bcanadd _cost) (CallFunction|ConditionandCostOfTile Position _output_get))
    (if _bcanadd
      (Utilities|Array|Add (LocalVariables|GetNeighbor) (Utilities|Struct|MakeST_PathfindingData (LocalVariables|GetAddPosition) _cost 99999 99999 Position))))
  (if (CallFunction|IsIntEven (LocalVariables|GetXValue))
    (for _index_2 (range 0 1)
      (LocalVariables|SetConsideredXValue (+ (* _index_2 2) -1 (LocalVariables|GetXValue)))
      (for _index_3 (range 0 1)
        (LocalVariables|SetConsideredYValue (- (LocalVariables|GetYValue) _index_3))
        (LocalVariables|SetAddPosition (Utilities|Struct|MakeIntPoint (LocalVariables|GetConsideredXValue) (LocalVariables|GetConsideredYValue)))
        (bind (_bcanadd_2 _cost_2) (CallFunction|ConditionandCostOfTile Position (LocalVariables|GetAddPosition)))
        (if _bcanadd_2
          (Utilities|Array|Add (LocalVariables|GetNeighbor) (Utilities|Struct|MakeST_PathfindingData (LocalVariables|GetAddPosition) _cost_2 99999 99999 Position)))))
    (return (LocalVariables|GetNeighbor))
    (else
      (for _index_4 (range 0 1)
        (LocalVariables|SetConsideredXValue (+ (* _index_4 2) -1 (LocalVariables|GetXValue)))
        (for _index_5 (range 0 1)
          (LocalVariables|SetConsideredYValue (+ (LocalVariables|GetYValue) _index_5))
          (LocalVariables|SetAddPosition (Utilities|Struct|MakeIntPoint (LocalVariables|GetConsideredXValue) (LocalVariables|GetConsideredYValue)))
          (bind (_bcanadd_3 _cost_3) (CallFunction|ConditionandCostOfTile Position (LocalVariables|GetAddPosition)))
          (if _bcanadd_3
            (Utilities|Array|Add (LocalVariables|GetNeighbor) (Utilities|Struct|MakeST_PathfindingData (LocalVariables|GetAddPosition) _cost_3 99999 99999 Position)))))
      (return (LocalVariables|GetNeighbor)))))

(fn ClearTiles
  (for _array_element (Variables|Default|GetValidNeighborPositions)
    (Default|RemoveStateTile (Variables|Default|GetGrid) (.position _array_element) "Neighbor"))
  (Utilities|Array|Clear (Variables|Default|GetValidNeighborPositions))
  (Components|InstancedStaticMesh|ClearInstances (Variables|Default|GetInstancedStaticMesh)))

(fn ConditionandCostOfTile
  (params (Position :type Int%20Point%20Structure) (NeighborToAdd :type Int%20Point%20Structure))
  (bind _grid (Variables|Default|GetGrid))
  (bind (_success _tiledata) (Default|GetTileData _grid NeighborToAdd))
  (return (Math|Boolean|ANDBoolean _success (or (GameplayTags|HasTag (.tiletags _tiledata) "(TagName=\"Grid.Type.Walkable\")") (GameplayTags|HasTag (.tiletags _tiledata) (select (Variables|Default|GetbFlyingUnit) "(TagName=\"Grid.Type.FlyingOnly\")" "(TagName=\"Grid.Type.Walkable\")"))) (!= Position NeighborToAdd) (Default|IsTileWalkable (Variables|Default|GetGrid) NeighborToAdd) (or (not (Utilities|IsValid (Utilities|Struct|BreakGridTileOccupancy (.occupancy _tiledata)))) (Variables|Default|GetbIgnoreUnit))) (Default|GetTileCostforPathfinding (Variables|Default|GetGrid) (Variables|Default|GetbFlyingUnit) (.tiletags _tiledata))))

(fn SetIsFlying
  (params (bFlying :type Boolean))
  (Variables|Default|SetbFlyingUnit bFlying))

(fn GetIsFlyingUnit
  (return (Variables|Default|GetbFlyingUnit)))

(fn GetValidTileTags
  (return (Variables|Default|GetValidTileTags)))

(fn SetIgnoreUnit
  (params (bIgnoreUnit :type Boolean))
  (Variables|Default|SetbIgnoreUnit bIgnoreUnit))