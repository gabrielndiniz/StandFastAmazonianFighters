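; Grid action that runs an A*-style search from a start tile to a target within a path cost budget, or returns reachable tiles.
; It keeps a cost-sorted discovered list, expands valid neighbors from ShowTileNeighbor, picks tiles via the grid's nearest-to-target query and backtracks the path.
; An optional delay steps the search through a gate.
; Tile states and instanced meshes visualize discovered, analyzed and path tiles.
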(event Custom|FindPathWithDelay
  (Utilities|FlowControl|Sequence
    (:then_0
      (goto _label_2 Open))
    (:then_1
      (if (> (Utilities|Array|Length (Variables|Default|GetDiscoveredTilePosition)) 0) :!label _label
        (bind _foundtargettile (CallFunction|AnalyseNextDiscoveredTile))
        (if _foundtargettile
          (bind _path (CallFunction|GeneratePath))
          (CallFunction|UpdateStatesonEnd _path)
          (Default|CallOnPathfindingCompleted)
          (else
            (Utilities|FlowControl|Delay (Variables|Default|GetDelayBetweenInterations))
            (Utilities|FlowControl|Gate true :!label _label_2
              (:Exit
                (goto _label)))))
        (else
          (CallFunction|UpdateStatesonEnd (Utilities|Array|MakeArray (Utilities|Struct|MakeIntPoint 99999 99999)))
          (Default|CallOnPathfindingCompleted))))))

(event Custom|CloseDelayGate
  (Utilities|FlowControl|Gate true) ; enters at Close
)

(event EventBeginPlay
  (bind _grid (Variables|Default|GetGrid))
  (bind _gridlastposition (Default|GetGridLastPosition _grid))
  (|CallParentFunction)
  (Utilities|IsValid (Variables|Default|GetGrid) :!label _label
    (:Is%20Valid
      ;[0.04688 0.04688 0.04688] To reduce chance of infinite loop.
      (Variables|Default|SetMaxExpectedInteractions (+ (.x _gridlastposition) (.y _gridlastposition))))
    (:Is%20Not%20Valid
      (Utilities|FlowControl|Delay 2.0)
      (goto _label))))

(event Collision|EventActorBeginOverlap
  (params (OtherActor :type Actor%20Object%20Reference))
  (|CallParentFunction OtherActor) ; This node is disabled and will not be called.\nDrag off pins to build functionality.
)

(event EventTick
  (params (DeltaSeconds :type Float%20%28single-precision%29))
  (|CallParentFunction DeltaSeconds) ; This node is disabled and will not be called.\nDrag off pins to build functionality.
)

(fn ConstructionScript
  (|CallParentFunction))

(fn ExecuteAction
  (params (Position%201 :type Int%20Point%20Structure) (bHitResult :type Boolean) (Position%202 :type Int%20Point%20Structure))
  (bind (_success _tiledata1 _tiledata2) (|CallParentFunction Position%201 bHitResult Position%202))
  (Utilities|IsValid (Variables|Default|GetGrid)
    (:Is%20Valid
      (if (!= Position%201 (Variables|Default|GetCurrentPositon))
        (CallFunction|ClearGeneratedData true)
        (if bHitResult
          (bind _path (CallFunction|FindPath Position%201 Position%202 false false true))
          (CallFunction|UpdateStatesonEnd _path))
        (return _success _tiledata1 _tiledata2)))
    (:Is%20Not%20Valid
      (return false "" ""))))

(fn SetShowTileNeighbor
  (params (ShowTileNeighbor :type BP%20Action%20Show%20Tile%20Neighbor%20Object%20Reference))
  (Variables|Default|SetShowTileNeighbor ShowTileNeighbor))

(fn SetShowPath
  (params (bShowPath :type Boolean))
  (Variables|Default|SetbShowPath bShowPath))

(fn ShowPath
  (bind _grid (Variables|Default|GetGrid))
  (bind _tiledata (Default|GetTileData _grid ""))
  (bind (_x _y _z) (Math|Vector|BreakVector (.worldlocation _tiledata)))
  (CallFunction|ClearInstances)
  (if (and (Variables|Default|GetbShowPath) (> (.x (Utilities|Array|Get(acopy) (Variables|Default|GetPath))) -999))
    (for _array_element (Variables|Default|GetPath)
      (Components|InstancedStaticMesh|AddInstance (Variables|Default|GetInstancedStaticMeshPath) (Math|Transform|MakeTransform (Math|Vector|MakeVector _x _y (+ _z 4.0)) "0, 0, 0" "1.000000,1.000000,1.000000") true))))

(fn FindPath
  (params (Start :type Int%20Point%20Structure) (Target :type Int%20Point%20Structure) (bReturnReachable :type Boolean) (IgnoreUnitOnTile :type Boolean) (bClearPath :type Boolean))
  (Utilities|FlowControl|Sequence
    (:then_0
      (CallFunction|ClearGeneratedData bClearPath)
      (bind _output_get (Variables|Default|SetIgnoreUnit IgnoreUnitOnTile))
      (Default|SetIgnoreUnit (Variables|Default|GetShowTileNeighbor) _output_get))
    (:then_1
      (Variables|Default|SetStartPosition Start)
      (Variables|Default|SetTargetPosition Target)
      (bind _bisvalid (CallFunction|IsInputDataValid))
      (if (or _bisvalid bReturnReachable)
        (bind _mincost (SettersAndGetters|GetMinimumCostBetweenTwoTiles Start Target))
        (if (or (>= (Variables|Default|GetPath%20Cost) _mincost) bReturnReachable)
          (CallFunction|DiscoverTile (Utilities|Struct|MakeST_PathfindingData Start 10 0 _mincost "(X=999,Y=999)"))
          (if (<= (Variables|Default|GetDelayBetweenInterations) 0.0)
            (while (> (Utilities|Array|Length (Variables|Default|GetDiscoveredTilePosition)) 0)
              (bind _foundtargettile (CallFunction|AnalyseNextDiscoveredTile))
              (if _foundtargettile
                (bind _path (CallFunction|GeneratePath))
                (Default|CallOnPathfindingCompleted)
                (return (select bReturnReachable (Variables|Default|GetAnalysedTilePositions) _path) true)))
            (Default|CallOnPathfindingCompleted)
            (return (select bReturnReachable (Variables|Default|GetAnalysedTilePositions) (Utilities|Array|MakeArray (Utilities|Struct|MakeIntPoint -999 -999))) false)
            (else
              (CallFunction|FindPathwithDelay)
              (return (select bReturnReachable (Variables|Default|GetAnalysedTilePositions) (Utilities|Array|MakeArray (Utilities|Struct|MakeIntPoint -999 -999))) false)))
          (else
            (Default|CallOnPathfindingCompleted)
            (return (select bReturnReachable (Variables|Default|GetAnalysedTilePositions) (Utilities|Array|MakeArray (Utilities|Struct|MakeIntPoint -999 -999))) false)))
        (else
          (Default|CallOnPathfindingCompleted)
          (return (select bReturnReachable (Variables|Default|GetAnalysedTilePositions) (Utilities|Array|MakeArray (Utilities|Struct|MakeIntPoint -999 -999))) false))))))

(fn IsInputDataValid
  (return (Math|Boolean|ANDBoolean (Default|IsTileWalkable (Variables|Default|GetGrid)) (Default|IsTileWalkable (Variables|Default|GetGrid)) (!= (Variables|Default|GetStartPosition) (Variables|Default|GetTargetPosition)) (or (not (Utilities|IsValid (Utilities|Struct|BreakGridTileOccupancy (.occupancy (.TileData (Default|GetTileData (Variables|Default|GetGrid))))))) (Variables|Default|GetIgnoreUnit)))))

(fn DiscoverTile
  (params (TilePathData :type ST%20Pathfinding%20Data%20Structure))
  (Utilities|Map|Add (Variables|Default|GetPathfindingData) (.Position (Utilities|Struct|BreakST_PathfindingData TilePathData)) TilePathData)
  (CallFunction|InsertTileinDiscoveredArray TilePathData))

(fn GetMinimumCostBetweenTwoTiles
  (params (Position1 :type Int%20Point%20Structure) (Position2 :type Int%20Point%20Structure))
  ;[0.05208 0.05208 0.05208] Modifying from the video. https://www.youtube.com/watch?v=xakl29fupCA&list=PLBLmKCAjA25CKFIvmaA8y3tsX_URgkX4O&index=30 TODO FIX: have problem when pathcost is 5.
  (return (Math|Float|Truncate (* (/ (Math|Vector|Distance(Vector) (.worldlocation (.TileData (Default|GetTileData (Variables|Default|GetGrid)))) (.worldlocation (.TileData (Default|GetTileData (Variables|Default|GetGrid))))) (LocalVariables|GetMinimumDistanceCenterTile)) (Math|Conversions|ToFloat(Integer) (Variables|Default|GetCorrectionFactor))))))

(fn AnalyseNextDiscoveredTile
  (Utilities|FlowControl|Sequence
    (:then_0
      (bind _tilepathdata (CallFunction|PullCheapestTileOutOfDiscoveredList))
      (bind _output_get (Variables|Default|SetCurrentDiscoveredTile _tilepathdata))
      (if (<= (.costfromstart _output_get) (Variables|Default|GetPath%20Cost))
        (bind _neighborpositions (Default|GetValidTileNeighbors (Variables|Default|GetShowTileNeighbor) (.position _output_get)))
        (Variables|Default|SetCurrentNeighbors _neighborpositions)
        (while (> (Utilities|Array|Length (Variables|Default|GetCurrentNeighbors)) 0)
          (bind _bistargettile (CallFunction|DiscoverNextNeighbor))
          (if _bistargettile
            (return true)))))
    (:then_1
      (return false))))

(fn GeneratePath
  (LocalVariables|SetCurrent (Variables|Default|GetTargetPosition))
  (while (and (!= (LocalVariables|GetCurrent) (Variables|Default|GetStartPosition)) (< (LocalVariables|GetCount) (Variables|Default|GetMaxExpectedInteractions)))
    (Utilities|Array|Add (LocalVariables|GetInvertedPath) (LocalVariables|GetCurrent))
    (LocalVariables|SetCurrent (.previousposition (.Value (Utilities|Map|Find (Variables|Default|GetPathfindingData) (LocalVariables|GetCurrent)))))
    (LocalVariables|SetCount (+ (LocalVariables|GetCount) 1)))
  (bind _arrayelement (Utilities|Array|ReverseforEachLoop (LocalVariables|GetInvertedPath))
    (:LoopBody
      (Utilities|Array|Add (LocalVariables|GetResult) _arrayelement))
    (:Completed
      (return (LocalVariables|GetResult)))))

(fn PullCheapestTileOutOfDiscoveredList
  (bind _grid (Variables|Default|GetGrid))
  (bind _tiledata (Default|GetTileData _grid))
  (bind (_x _y _z) (Math|Vector|BreakVector (.worldlocation _tiledata)))
  (bind _index (Default|GetNearestTilefromTarget :self (Variables|Default|GetGrid) :ConsiderFlying (Default|GetIsFlyingUnit (Variables|Default|GetShowTileNeighbor))))
  (LocalVariables|SetIndexToUse _index)
  (LocalVariables|SetTilePosition (Utilities|Array|Get(acopy) (Variables|Default|GetDiscoveredTilePosition) (LocalVariables|GetIndexToUse)))
  (Utilities|Array|RemoveIndex (Variables|Default|GetDiscoveredTileSortingCosts) (LocalVariables|GetIndexToUse))
  (Utilities|Array|RemoveIndex (Variables|Default|GetDiscoveredTilePosition) (LocalVariables|GetIndexToUse))
  (Utilities|Array|Add (Variables|Default|GetAnalysedTilePositions) (LocalVariables|GetTilePosition))
  (Utilities|FlowControl|Sequence
    (:then_0
      (if (Variables|Default|GetbShowAnalizedTiles)
        (Default|RemoveStateTile :self (Variables|Default|GetGrid) :Tile%20State "Discovered")
        (Default|AddStateTile :self (Variables|Default|GetGrid))
        (Components|InstancedStaticMesh|AddInstance (Variables|Default|GetInstancedStaticMeshAnalized) (Math|Transform|MakeTransform (Math|Vector|MakeVector _x _y (+ _z 2.0)) "0, 0, 0" "1.000000,1.000000,1.000000") false)))
    (:then_1
      (return (.Value (Utilities|Map|Find (Variables|Default|GetPathfindingData) (LocalVariables|GetTilePosition)))))))

(fn DiscoverNextNeighbor
  (bind _currentdiscoveredtile (Variables|Default|GetCurrentDiscoveredTile))
  (bind (_position _costtoentertile _costfromstart) (Utilities|Struct|BreakST_PathfindingData _currentdiscoveredtile))
  (Utilities|FlowControl|Sequence
    (:then_0
      (Variables|Default|SetCurrentNeighbor (Utilities|Array|Get(acopy) (Variables|Default|GetCurrentNeighbors)))
      (Utilities|Array|RemoveIndex (Variables|Default|GetCurrentNeighbors))
      (if (and (not (Utilities|Array|ContainsItem (Variables|Default|GetAnalysedTilePositions) (.position (Variables|Default|GetCurrentNeighbor)))) (Math|Boolean|ORBoolean (Utilities|IsValid (Utilities|Struct|BreakGridTileOccupancy (.occupancy (.TileData (Default|GetTileData (Variables|Default|GetGrid)))))) (!= (Variables|Default|GetStartPosition) (.position (Variables|Default|GetCurrentNeighbor))) (Variables|Default|GetIgnoreUnit)))
        (bind _output_get (LocalVariables|SetCostFromStart (+ _costfromstart (+ (* (.CostToEnterTile (Utilities|Struct|BreakST_PathfindingData (Variables|Default|GetCurrentNeighbor))) 10) (* (Math|Conversions|ToInteger(Boolean) (CallFunction|IsintheSameLine _position (.Position (Utilities|Struct|BreakST_PathfindingData (Variables|Default|GetCurrentNeighbor))))) 4)))))
        (if (<= _output_get (Variables|Default|GetPath%20Cost))
          (bind _output_get_2 (LocalVariables|SetIndexDiscovered (Utilities|Array|FindItem (Variables|Default|GetDiscoveredTilePosition) (.position (Variables|Default|GetCurrentNeighbor)))))
          (if (== _output_get_2 -1)
            (bind _mincost (SettersAndGetters|GetMinimumCostBetweenTwoTiles (.Position (Utilities|Struct|BreakST_PathfindingData (Variables|Default|GetCurrentNeighbor))) (Variables|Default|GetTargetPosition) :!label _label))
            (CallFunction|DiscoverTile (Utilities|Struct|MakeST_PathfindingData (.Position (Utilities|Struct|BreakST_PathfindingData (Variables|Default|GetCurrentNeighbor))) (.CostToEnterTile (Utilities|Struct|BreakST_PathfindingData (Variables|Default|GetCurrentNeighbor))) (LocalVariables|GetCostFromStart) _mincost (.position (Variables|Default|GetCurrentDiscoveredTile))))
            (if (Class|KismetMathLibrary|EqualIntPointIntPoint (.Position (Utilities|Struct|BreakST_PathfindingData (Variables|Default|GetCurrentNeighbor))) (Variables|Default|GetTargetPosition))
              (return true))
            (else
              (bind _output_get_3 (Variables|Default|SetCurrentNeighbor (.Value (Utilities|Map|Find (Variables|Default|GetPathfindingData) (.position (Variables|Default|GetCurrentNeighbor))))))
              (if (< (LocalVariables|GetCostFromStart) (.costfromstart _output_get_3))
                (Utilities|Array|RemoveIndex (Variables|Default|GetDiscoveredTilePosition) (LocalVariables|GetIndexDiscovered))
                (Utilities|Array|RemoveIndex (Variables|Default|GetDiscoveredTileSortingCosts) (LocalVariables|GetIndexDiscovered))
                (goto _label)))))))
    (:then_1
      (return false))))

(fn InsertTileinDiscoveredArray
  (params (TileData :type ST%20Pathfinding%20Data%20Structure))
  (bind _grid (Variables|Default|GetGrid))
  (bind _discoveredtilesortingcosts (Variables|Default|GetDiscoveredTileSortingCosts))
  (bind _tiledata (Default|GetTileData _grid))
  (bind (_x _y _z) (Math|Vector|BreakVector (.worldlocation _tiledata)))
  (Utilities|FlowControl|Sequence
    (:then_0
      (if (Variables|Default|GetbShowDiscoveredTiles)
        (Default|AddStateTile :self (Variables|Default|GetGrid) :GridTileState "Discovered")
        (Components|InstancedStaticMesh|AddInstance (Variables|Default|GetInstancedStaticMeshDiscover) (Math|Transform|MakeTransform (Math|Vector|MakeVector _x _y (+ _z 1.0)) "0, 0, 0" "1.000000,1.000000,1.000000") false)))
    (:then_1
      (LocalVariables|SetSortingCost (SettersAndGetters|GetTileSortingCost TileData))
      (if (== (Utilities|Array|Length (Variables|Default|GetDiscoveredTileSortingCosts)) 0)
        (Utilities|Array|Add (Variables|Default|GetDiscoveredTileSortingCosts) (LocalVariables|GetSortingCost) :!label _label)
        (Utilities|Array|Add (Variables|Default|GetDiscoveredTilePosition) (.position TileData))
        (elif (>= (LocalVariables|GetSortingCost) (Utilities|Array|Get(acopy) _discoveredtilesortingcosts (Utilities|Array|LastIndex _discoveredtilesortingcosts)))
          (goto _label)
          (else
            (bind (_array_element _array_index) (Utilities|Array|ForEachLoopwithBreak (Variables|Default|GetDiscoveredTileSortingCosts) :!label _label_2)
              (:LoopBody
                (LocalVariables|SetIndexToConsider _array_index)
                (if (>= _array_element (LocalVariables|GetSortingCost))
                  (Utilities|Array|Insert (Variables|Default|GetDiscoveredTileSortingCosts) (LocalVariables|GetSortingCost) (LocalVariables|GetIndexToConsider))
                  (Utilities|Array|Insert (Variables|Default|GetDiscoveredTilePosition) (.position TileData) (LocalVariables|GetIndexToConsider))
                  (goto _label_2 Break))))))))))

(fn ClearGeneratedData
  (params (ClearPath :type Boolean))
  (Utilities|Array|Clear (Variables|Default|GetDiscoveredTilePosition))
  (Utilities|Array|Clear (Variables|Default|GetDiscoveredTileSortingCosts))
  (Utilities|Array|Clear (Variables|Default|GetDiscoveredTilePosition))
  (Utilities|Array|Clear (Variables|Default|GetAnalysedTilePositions))
  (if ClearPath
    (for _array_element (Variables|Default|GetPath)
      (Default|RemoveStateTile :self (Variables|Default|GetGrid) :Tile%20State "InPath"))
    (Utilities|Array|Clear (Variables|Default|GetPath))
    (Components|InstancedStaticMesh|ClearInstances (Variables|Default|GetInstancedStaticMeshPath))
    (Components|InstancedStaticMesh|ClearInstances (Variables|Default|GetInstancedStaticMeshDiscover))
    (Components|InstancedStaticMesh|ClearInstances (Variables|Default|GetInstancedStaticMeshAnalized))
    (Default|CallOnPathfindingCleared)))

(fn GetPathfindingData
  (return (Variables|Default|GetPathfindingData)))

(fn GetDiscoveredTiles
  (return (Variables|Default|GetDiscoveredTilePosition) (Variables|Default|GetDiscoveredTileSortingCosts)))

(fn SetShowDiscoveredTiles
  (params (bShowDiscoveredTiles :type Boolean))
  (bind _grid (Variables|Default|GetGrid))
  (bind _tiledata (Default|GetTileData _grid ""))
  (bind (_x _y _z) (Math|Vector|BreakVector (.worldlocation _tiledata)))
  (bind _output_get (Variables|Default|SetbShowDiscoveredTiles bShowDiscoveredTiles))
  (if _output_get
    (for _array_element (Variables|Default|GetDiscoveredTilePosition)
      (Default|AddStateTile :self (Variables|Default|GetGrid) :GridTileState "Discovered")
      (Components|InstancedStaticMesh|AddInstance (Variables|Default|GetInstancedStaticMeshDiscover) (Math|Transform|MakeTransform (Math|Vector|MakeVector _x _y (+ _z 1.0)) "0, 0, 0" "1.000000,1.000000,1.000000") false))
    (else
      (Components|InstancedStaticMesh|ClearInstances (Variables|Default|GetInstancedStaticMeshDiscover))
      (for _array_element_2 (Variables|Default|GetDiscoveredTilePosition)
        (Default|RemoveStateTile :self (Variables|Default|GetGrid) :Tile%20State "Discovered")))))

(fn SetShowAnalizedTiles
  (params (bShowAnalizedTiles :type Boolean))
  (bind _grid (Variables|Default|GetGrid))
  (bind _tiledata (Default|GetTileData _grid ""))
  (bind _output_get (Variables|Default|SetbShowAnalizedTiles bShowAnalizedTiles))
  (if _output_get
    (for _array_element (Variables|Default|GetAnalysedTilePositions)
      (Default|AddStateTile :self (Variables|Default|GetGrid) :GridTileState "Analyzed")
      (Components|InstancedStaticMesh|AddInstance (Variables|Default|GetInstancedStaticMeshAnalized) (Math|Transform|MakeTransform (Math|Vector|MakeVector (.x (.worldlocation _tiledata)) (.y (.worldlocation _tiledata)) (+ (.z (.worldlocation _tiledata)) 2.0)) "0, 0, 0" "1.000000,1.000000,1.000000") false))
    (else
      (Components|InstancedStaticMesh|ClearInstances (Variables|Default|GetInstancedStaticMeshAnalized))
      (for _array_element_2 (Variables|Default|GetAnalysedTilePositions)
        (Default|RemoveStateTile :self (Variables|Default|GetGrid) :Tile%20State "Analyzed")))))

(fn SetDelayBetweenInterations
  (params (DelayBetweenInterations :type Float%20%28double-precision%29))
  (bind _output_get (Variables|Default|SetDelayBetweenInterations DelayBetweenInterations))
  (if (== _output_get 0.0)
    (CallFunction|CloseDelayGate)))

(fn UpdateStatesonEnd
  (params (Path :type Array%20of%20Int%20Point%20Structures))
  (bind _output_get (Variables|Default|SetPath Path))
  (for _array_element _output_get
    (Default|AddStateTile :self (Variables|Default|GetGrid) :GridTileState "InPath")
    (CallFunction|ShowPath)))

(fn GetTileSortingCost
  (params (ST_PathfindingData :type ST%20Pathfinding%20Data%20Structure%20%28by%20ref%29))
  (bind (_position _costtoentertile _costfromstart _minimumcosttotarget) (Utilities|Struct|BreakST_PathfindingData ST_PathfindingData))
  (return (+ _costfromstart _minimumcosttotarget)))

(fn GetPath
  (return (Variables|Default|GetPath)))

(fn SetPathCost
  (params (Path%20Cost :type Integer))
  (Variables|Default|SetPath%20Cost (* Path%20Cost (Variables|Default|GetCorrectionFactor))))

(fn GetPathCost
  (return (Variables|Default|GetPath%20Cost)))

(fn GetActualCostfromPath
  (params (ActualPath :type Array%20of%20Int%20Point%20Structures) (bIsFlyingUnit :type Boolean))
  (bind _grid (Variables|Default|GetGrid))
  (Utilities|FlowControl|Sequence
    (:then_0
      (Variables|Default|SetActualCostFromStart 0)
      (if bIsFlyingUnit
        (Variables|Default|SetActualCostFromStart (Utilities|Array|Length ActualPath))
        (else
          (for _array_element ActualPath
            (Variables|Default|SetActualCostFromStart (+ (Default|GetTileCostforPathfinding _grid false (.TileTags (Utilities|Struct|BreakGridTileStaticData (.TileData (Default|GetTileData _grid ""))))) (Variables|Default|GetActualCostFromStart)))))))
    (:then_1
      (return (Variables|Default|GetActualCostFromStart)))))

(fn ClearInstances
  (Components|InstancedStaticMesh|ClearInstances (Variables|Default|GetInstancedStaticMeshPath)))