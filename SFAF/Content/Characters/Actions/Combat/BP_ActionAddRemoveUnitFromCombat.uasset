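; Grid action that adds or removes combat units on a tile, switched by IsAddingUnit.
; Adding spawns the combatant class looked up from UnitDatabase by type tag on a walkable tile, then registers it with the CombatSystem using the configured team and AI flag.
; Removing takes the tile's occupying unit out of combat and destroys it.
; BeginPlay retries every second until it finds BP_CombatSystem.
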(event EventBeginPlay
  (|CallParentFunction)
  (bind _returnvalue (Actor|GetActorOfClass "/Game/Combat/BP_CombatSystem.BP_CombatSystem_C" :!label _label))
  (bind _output_get (Variables|Default|SetCombatSystem _returnvalue))
  (Utilities|IsValid _output_get
    (:Is%20Not%20Valid
      (Utilities|FlowControl|Delay 1.0)
      (goto _label))))

(event Collision|EventActorBeginOverlap
  (params (OtherActor :type Actor%20Object%20Reference))
  (|CallParentFunction OtherActor) ; This node is disabled and will not be called.\nDrag off pins to build functionality.
)

(event EventTick
  (params (DeltaSeconds :type Float%20%28single-precision%29)))

(fn ConstructionScript
  (|CallParentFunction))

(fn GetIsAddingUnit
  (return (Variables|Default|GetbIsAddingUnit)))

(fn SetIsAddingUnit
  (params (bIsAddingUnit :type Boolean))
  (Variables|Default|SetbIsAddingUnit bIsAddingUnit))

(fn ExecuteAction
  (params (Position%201 :type Int%20Point%20Structure) (bHitResult :type Boolean) (Position%202 :type Int%20Point%20Structure))
  (bind (_success _tiledata1 _tiledata2) (|CallParentFunction Position%201 bHitResult Position%202))
  (if (Variables|Default|GetbIsAddingUnit)
    (CallFunction|AddUnit Position%201 true)
    (else
      (CallFunction|RemoveUnit Position%201)))
  (return _success _tiledata1 _tiledata2))

(fn AddUnit
  (params (Position%201 :type Int%20Point%20Structure) (bAddToActiveList :type Boolean))
  (if (Default|IsTileWalkable (Variables|Default|GetGrid) Position%201)
    (bind _returnvalue (Game|SpawnActorfromClass (.CombatantClass (Utilities|Struct|BreakCombatantData (.OutData (Class|CombatantDatabaseDataAsset|GetCombatantData (Variables|Default|GetUnitDatabase) (Variables|Default|GetUnitTypeTag))))) (Math|Transform|MakeTransform "0.000000,0.000000,99999.000000" "0, 0, 0" "1.000000,1.000000,1.000000") "Undefined" "SelectDefaultAtRuntime" 0 0))
    (bind _asbp_combatant_base (Utilities|Casting|CastToBP_Combatant_Base _returnvalue))
    (Default|AddUnitinCombat (Variables|Default|GetCombatSystem) _asbp_combatant_base Position%201 (Variables|Default|GetbUseAI) bAddToActiveList)
    (Default|SetUnitTeamNumber (Variables|Default|GetCombatSystem) _asbp_combatant_base (Variables|Default|GetTeamNumber))
    (return _asbp_combatant_base)
    (else
      (return 0))))

(fn RemoveUnit
  (params (Position%201 :type Int%20Point%20Structure))
  (bind _grid (Variables|Default|GetGrid))
  (bind (_success _tiledata) (Default|GetTileData _grid Position%201))
  (bind _asbp_combatant_base (Utilities|Casting|CastToBP_Combatant_Base (Utilities|Struct|BreakGridTileOccupancy (.occupancy _tiledata))))
  (if (and (Utilities|IsValid _asbp_combatant_base) _success)
    (Default|RemoveUnitfromCombat (Variables|Default|GetCombatSystem) _asbp_combatant_base true)
    (Default|SetUnitTeamNumber (Variables|Default|GetCombatSystem) _asbp_combatant_base 255)))

(fn SetTeamNumber
  (params (TeamNumber :type Byte))
  (Variables|Default|SetTeamNumber TeamNumber))

(fn SetUseAI
  (params (bUseAI :type Boolean))
  (Variables|Default|SetbUseAI bUseAI))

(fn GetUseAI
  (return (Variables|Default|GetbUseAI)))

(fn SetUnitTypeTag
  (params (UnitTypeTag :type Gameplay%20Tag%20Structure))
  (Variables|Default|SetUnitTypeTag UnitTypeTag))

(fn GetUnitTypeTag
  (return (Variables|Default|GetUnitTypeTag)))