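; Grid combat action that previews a spell's range and area of effect, then hands casting to BP_CombatSystem.
; FindRequiredPositions builds both patterns from reachable-tile searches, filtered by minimum reach, line shape, line-of-sight traces and target requirement.
; Instanced static meshes display the tiles, with the area following the hovered tile while it is in range.
; ExecuteAction casts only when the target lies within the computed range.
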(event EventBeginPlay
  (|CallParentFunction)
  (bind _returnvalue (Actor|GetActorOfClass "/Game/Combat/BP_CombatSystem.BP_CombatSystem_C" :!label _label))
  (bind _output_get (Variables|Default|SetCombatSystem _returnvalue))
  (Utilities|IsValid _output_get
    (:Is%20Not%20Valid
      (Utilities|FlowControl|Delay 1.0)
      (goto _label))))

(event Collision|EventActorBeginOverlap
  (params (OtherActor :type Actor%20Object%20Reference))
  (|CallParentFunction OtherActor) ; This node is disabled and will not be called.\nDrag off pins to build functionality.
)

(event EventTick
  (params (DeltaSeconds :type Float%20%28single-precision%29)))

(fn ConstructionScript
  (|CallParentFunction))

(fn GetIsCastingSpell
  (return (Variables|Default|GetbIsCastingSpell)))

(fn SetIsCastingSpell
  (params (bIsCastingSpell :type Boolean) (ActionManager :type BP%20Action%20Manager%20Object%20Reference))
  (bind _grid (Variables|Default|GetGrid))
  (Variables|Default|SetbIsCastingSpell bIsCastingSpell)
  (Variables|Default|SetAction%20Manager ActionManager)
  (if (Variables|Default|GetbIsCastingSpell)
    (CallFunction|ShowSpellRangePattern)
    (CallFunction|ShowSpellAOEPattern)
    (Variables|Default|SetOriginPosition (.SelectedPosition (Default|GetSelectedTile ActionManager)))
    (Default|SetShowReachables (Variables|/Game/TopDown/Blueprints/BP_ActionManager.BP_ActionManager_C|GetSelectTile ActionManager) false)
    (else
      (Components|InstancedStaticMesh|ClearInstances (Variables|Default|GetInstancedStaticMeshSpellRange))
      (if (> (.x (Variables|Default|GetOriginPosition)) -999)
        (Default|SetTiletoHover ActionManager _grid false (.worldlocation (.TileData (Default|GetTileData _grid))))
        (Default|SetSelectedTile ActionManager false)
        (Variables|Default|SetOriginPosition (Utilities|Struct|MakeIntPoint -999 -999))))))

(fn GetSpell
  (return (Variables|Default|GetRangeType)))

(fn SetSpellRangeType
  (params (SpellRangeType :type E_Spell%20Enum :default "NewEnumerator0"))
  (Variables|Default|SetRangeType SpellRangeType))

(fn ExecuteAction
  (params (Position%201 :type Int%20Point%20Structure) (bHitResult :type Boolean) (Position%202 :type Int%20Point%20Structure))
  (bind (_success _tiledata1 _tiledata2) (|CallParentFunction Position%201 bHitResult Position%202))
  (bind _output_get (LocalVariables|SetbOkToCast (Math|Boolean|ANDBoolean (Variables|Default|GetbIsCastingSpell) (Utilities|Enum|NotEqual(Enum) (Variables|Default|GetRangeType) "NewEnumerator0") (Utilities|Array|ContainsItem (Variables|Default|GetPositionsInRange) Position%202))))
  (if _output_get
    (Default|CastSpell (Variables|Default|GetCombatSystem) (Variables|Default|GetRangeType) (Variables|Default|GetAOE%20Type) (Variables|Default|GetSpellEffectType) Position%201 Position%202 (Variables|Default|GetPositionsInAOE) (Variables|Default|GetImpact))
    (return (and (LocalVariables|GetbOkToCast) _success) _tiledata1 _tiledata2)))

(fn ShowSpellRangePattern
  (bind (_positions _success) (CallFunction|FindRequiredPositions (Variables|Default|GetRangeDataCast) (Variables|Default|GetRangeType) (Variables|Default|GetOriginPosition)))
  (bind _output_get (Variables|Default|SetPositionsInRange _positions))
  (bind _erasepositions (CallFunction|InstantiatePatterninPositions _output_get _success (Variables|Default|GetInstancedStaticMeshSpellRange) 4.0))
  (if _erasepositions
    (Utilities|Array|Clear (Variables|Default|GetPositionsInRange))
    (Utilities|Array|Add (Variables|Default|GetPositionsInRange) (Utilities|Struct|MakeIntPoint -999 -999))))

(fn SetSpellRangePattern
  (params (RangeDataCast :type ST%20Spell%20Data%20Cast%20Structure))
  (Variables|Default|SetRangeDataCast RangeDataCast)
  (if (Variables|Default|GetbIsCastingSpell)
    (CallFunction|ShowSpellRangePattern)
    (CallFunction|ShowSpellAOEPattern)))

(fn FindRequiredPositions
  (params (SpellDataCast :type ST%20Spell%20Data%20Cast%20Structure%20%28by%20ref%29) (SpellType :type E_Spell%20Enum%20%28by%20ref%29 :default "NewEnumerator0") (StartPosition :type Int%20Point%20Structure%20%28by%20ref%29))
  (bind _array (Utilities|Array|MakeArray (Utilities|Struct|MakeIntPoint -999 -999)))
  (bind _action_manager (Variables|Default|GetAction%20Manager))
  (bind _action_manager_2 (Variables|Default|GetAction%20Manager))
  (bind _findpathtotitle (Variables|/Game/TopDown/Blueprints/BP_ActionManager.BP_ActionManager_C|GetFindPathToTitle _action_manager))
  (bind _findpathtotitle_2 (Variables|/Game/TopDown/Blueprints/BP_ActionManager.BP_ActionManager_C|GetFindPathToTitle _action_manager_2))
  ;[0.07812 0.07812 0.07812] First, checking if function can continue.
  (if (Math|Boolean|ORBoolean (> (.x (.reachminmax SpellDataCast)) (.y (.reachminmax SpellDataCast))) (< (.y (.reachminmax SpellDataCast)) 0) (not (Utilities|IsValid (Variables|Default|GetAction%20Manager))) (Utilities|Enum|Equal(Enum) (.pattern SpellDataCast) "NewEnumerator0") (== SpellType 0))
    (return _array false false _array)
    (else
      (Default|SetSelectedFlyingUnit (Variables|Default|GetAction%20Manager) (.bisaerial SpellDataCast))
      ;[0.08854 0.08854 0.08854] Getting what is inside Range Y
      (Default|SetPathCost _findpathtotitle_2 (.y (.reachminmax SpellDataCast)))
      (bind _path (Default|FindPath _findpathtotitle_2 StartPosition (Utilities|Struct|MakeIntPoint -999 -999) true true true))
      (LocalVariables|SetPositionsInY _path)
      ;[0.08854 0.08854 0.08854] X = 0 -> Can Self-Cast, X = 1 -> Cannot Self-Cast
      (if (> (.x (.reachminmax SpellDataCast)) 1)
        (Default|SetPathCost _findpathtotitle (- (.x (.reachminmax SpellDataCast)) 1))
        (bind _path_2 (Default|FindPath _findpathtotitle StartPosition (Utilities|Struct|MakeIntPoint -999 -999) true true true))
        (LocalVariables|SetPositionsInX _path_2)
        (for _array_element (LocalVariables|GetPositionsInX)
          (if (Utilities|Array|ContainsItem (LocalVariables|GetPositionsInY) _array_element)
            (Utilities|Array|RemoveItem (LocalVariables|GetPositionsInY) _array_element))))
      ;[0.07812 0.07812 0.07812] Different Patterns Have Different Positions
      (switch Utilities|FlowControl|Switch|SwitchonE_SpellRangePattern (.pattern SpellDataCast)
        (:NewEnumerator0
          (if (.brequirelineofsight SpellDataCast) :!label _label
            (CallFunction|RemovePositionsWithoutLineOfSight StartPosition (.heightfromground SpellDataCast) (LocalVariables|GetPositionsInY) (.bdrawdebugline SpellDataCast)))
          (if (== (.x (.reachminmax SpellDataCast)) 0)
            (Utilities|Array|Add (LocalVariables|GetPositionsInY) StartPosition)
            (else
              (Utilities|Array|RemoveItem (LocalVariables|GetPositionsInY) StartPosition)))
          (bind (_bhittarget _unitshitspositions) (CallFunction|PositionsDoesHitATarget (LocalVariables|GetPositionsInY) StartPosition))
          (LocalVariables|SetbHitATarget _bhittarget)
          (LocalVariables|SetHitsPositions _unitshitspositions)
          (Utilities|FlowControl|Sequence ; Choosing what kind of Target Requirement needed.
            (:then_0
              (if (Utilities|Enum|Equal(Enum) (.TargetRequirement (Utilities|Struct|BreakST_SpellData_Cast SpellDataCast)) "NewEnumerator2")
                (return (LocalVariables|GetPositionsInY) (> (Utilities|Array|Length (LocalVariables|GetPositionsInY)) 0) (LocalVariables|GetbHitATarget) (LocalVariables|GetHitsPositions))))
            (:then_1
              (if (Utilities|Enum|Equal(Enum) (.TargetRequirement (Utilities|Struct|BreakST_SpellData_Cast SpellDataCast)) "NewEnumerator0")
                (return (LocalVariables|GetHitsPositions) (> (Utilities|Array|Length (LocalVariables|GetHitsPositions)) 0) (LocalVariables|GetbHitATarget) (LocalVariables|GetHitsPositions))))
            (:then_2
              (if (Utilities|Enum|Equal(Enum) (.TargetRequirement (Utilities|Struct|BreakST_SpellData_Cast SpellDataCast)) "NewEnumerator1")
                (for _array_element_2 (LocalVariables|GetHitsPositions)
                  (bind _returnvalue (Utilities|Array|RemoveItem (LocalVariables|GetPositionsInY) _array_element_2))
                  (if _returnvalue
                    (bind (_empty _outposition) (CallFunction|ClosestPosition _array_element_2 StartPosition))
                    (if _empty
                      (Utilities|Array|Add (LocalVariables|GetClosestsPositionFromHit) _outposition))))
                (return (LocalVariables|GetPositionsInY) (> (Utilities|Array|Length (LocalVariables|GetPositionsInY)) 0) (LocalVariables|GetbHitATarget) (LocalVariables|GetClosestsPositionFromHit))))))
        (:NewEnumerator1
          (bind (_arrayindex _arrayelement) (Utilities|Array|ReverseforEachLoop (LocalVariables|GetPositionsInY))
            (:LoopBody
              (if (not (CallFunction|IsintheSameLine _arrayelement StartPosition))
                (Utilities|Array|RemoveIndex (LocalVariables|GetPositionsInY) _arrayindex)))
            (:Completed
              (goto _label))))
        (:NewEnumerator7
          (goto _label))))))

(fn HasLineOfSight
  (params (StartPosition :type Int%20Point%20Structure) (TargetPosition :type Int%20Point%20Structure) (UnitHeight :type Float%20%28double-precision%29) (OffSetFromCenter :type Float%20%28double-precision%29) (bDrawDebugLine :type Boolean))
  (LocalVariables|SetStartTile "")
  (LocalVariables|SetTargetTile "")
  (LocalVariables|SetAdjustVector (Math|Vector|MakeVector 0.0 0.0 UnitHeight))
  (LocalVariables|SetStartLocation (+ (.worldlocation (LocalVariables|GetStartTile)) (LocalVariables|GetAdjustVector)))
  (LocalVariables|SetTargetLocation (+ (.worldlocation (LocalVariables|GetTargetTile)) (LocalVariables|GetAdjustVector)))
  (bind _returnvalue (Collision|LineTraceByChannel (LocalVariables|GetStartLocation) (LocalVariables|GetTargetLocation) "TraceTypeQuery6" false (Utilities|Array|MakeArray (Utilities|Struct|BreakGridTileOccupancy (.occupancy (LocalVariables|GetStartTile))) (Utilities|Struct|BreakGridTileOccupancy (.occupancy (LocalVariables|GetTargetTile)))) (select bDrawDebugLine "ForDuration" "None")))
  (LocalVariables|SetBlocked _returnvalue)
  (if (and (!= OffSetFromCenter 0.0) (LocalVariables|GetBlocked))
    (for _array_element (Utilities|Array|MakeArray (+ (LocalVariables|GetTargetLocation) (Math|Vector|MakeVector OffSetFromCenter 0.0 0.0)) (+ (LocalVariables|GetTargetLocation) (Math|Vector|MakeVector (* OffSetFromCenter -1.0) 0.0 0.0)) (+ (LocalVariables|GetTargetLocation) (Math|Vector|MakeVector 0.0 OffSetFromCenter 0.0)) (+ (LocalVariables|GetTargetLocation) (Math|Vector|MakeVector 0.0 (* OffSetFromCenter -1.0) 0.0)))
      (bind _returnvalue_2 (Collision|LineTraceByChannel (LocalVariables|GetStartLocation) (LocalVariables|GetTargetLocation) "TraceTypeQuery6" false (Utilities|Array|MakeArray (Utilities|Struct|BreakGridTileOccupancy (.occupancy (LocalVariables|GetStartTile))) (Utilities|Struct|BreakGridTileOccupancy (.occupancy (LocalVariables|GetTargetTile)))) (select bDrawDebugLine "ForDuration" "None")))
      (if (not _returnvalue_2)
        (return true)))
    (return false)
    (else
      (return (not (LocalVariables|GetBlocked))))))

(fn RemovePositionsWithoutLineOfSight
  (params (StartPosition :type Int%20Point%20Structure) (UnitHeight :type Float%20%28double-precision%29) (TargetPositions :type Array%20of%20Int%20Point%20Structures) (bDrawDebugLine :type Boolean))
  (bind (_arrayindex _arrayelement) (Utilities|Array|ReverseforEachLoop TargetPositions)
    (:LoopBody
      (if (not (CallFunction|HasLineOfSight StartPosition _arrayelement UnitHeight 0.0 bDrawDebugLine))
        (Utilities|Array|RemoveIndex TargetPositions _arrayindex)))))

(fn SetSpellAOEType
  (params (Spell%20AOE%20Type :type E_Spell%20Enum :default "NewEnumerator0"))
  (Variables|Default|SetAOE%20Type Spell%20AOE%20Type))

(fn SetSpellAOEPattern
  (params (AOE%20DataCast :type ST%20Spell%20Data%20Cast%20Structure))
  (Variables|Default|SetAOE%20DataCast AOE%20DataCast)
  (if (Variables|Default|GetbIsCastingSpell)
    (CallFunction|ShowSpellRangePattern)))

(fn ShowSpellAOEPattern
  (if true
    (bind (_positions _success) (CallFunction|FindRequiredPositions (Variables|Default|GetAOE%20DataCast) (Variables|Default|GetAOE%20Type) (Variables|Default|GetHovered%20Position)))
    (bind _output_get (Variables|Default|SetPositionsInAOE _positions))
    (bind _erasepositions (CallFunction|InstantiatePatterninPositions _output_get _success (Variables|Default|GetInstancedStaticMeshSpellAreaOfEffect) 5.0))
    (if _erasepositions
      (Utilities|Array|Clear (Variables|Default|GetPositionsInAOE))
      (Utilities|Array|Add (Variables|Default|GetPositionsInAOE) (Utilities|Struct|MakeIntPoint -999 -999)))
    (else
      (Components|InstancedStaticMesh|ClearInstances (Variables|Default|GetInstancedStaticMeshSpellAreaOfEffect)))))

(fn HoveredPosition
  (params (Position :type Int%20Point%20Structure))
  (if (Utilities|Array|ContainsItem (Variables|Default|GetPositionsInRange) Position)
    (Variables|Default|SetHovered%20Position Position)
    (CallFunction|ShowSpellAOEPattern)
    (else
      (Variables|Default|SetHovered%20Position (Variables|Default|GetOriginPosition))
      (CallFunction|ShowSpellAOEPattern))))

(fn InstantiatePatterninPositions
  (params (Positions :type Array%20of%20Int%20Point%20Structures) (Success :type Boolean) (InstancedStaticMeshs :type Instanced%20Static%20Mesh%20Component%20Object%20Reference) (CorrectionHeight :type Float%20%28double-precision%29))
  (bind _grid (Variables|Default|GetGrid))
  (bind _tiledata (Default|GetTileData _grid ""))
  (bind (_x _y _z) (Math|Vector|BreakVector (.worldlocation _tiledata)))
  (if Success
    (if (> (.x (Utilities|Array|Get(acopy) Positions)) -999)
      (Components|InstancedStaticMesh|ClearInstances InstancedStaticMeshs)
      (for _array_element Positions
        (Components|InstancedStaticMesh|AddInstance InstancedStaticMeshs (Math|Transform|MakeTransform (Math|Vector|MakeVector _x _y (+ _z CorrectionHeight)) "0, 0, 0" "1.000000,1.000000,1.000000") true))
      (return false)
      (else
        (return true)))
    (else
      (Components|InstancedStaticMesh|ClearInstances InstancedStaticMeshs)
      (return true))))

(fn SetSpellImpact
  (params (Impact :type ST%20Spell%20Data%20Impact%20Structure))
  (Variables|Default|SetImpact Impact))

(fn SetActionManager
  (params (Action%20Manager :type BP%20Action%20Manager%20Object%20Reference))
  (Variables|Default|SetAction%20Manager Action%20Manager))

(fn PositionsDoesHitATarget
  (params (Positions :type Array%20of%20Int%20Point%20Structures) (StartPosition :type Int%20Point%20Structure))
  (bind _combatsystem (Variables|Default|GetCombatSystem))
  (bind (_units _innactiveunits) (Default|GetUnits _combatsystem))
  (if (> (Utilities|Array|Length Positions) 0)
    (for _array_element _units
      (Utilities|IsValid _array_element
        (:Is%20Valid
          (if (!= (Default|GetPosition _array_element) StartPosition)
            (bind _output_get (LocalVariables|SetAnalyzedPosition (Default|GetPosition _array_element)))
            (if (Utilities|Array|ContainsItem Positions _output_get)
              (Utilities|Array|AddUnique (LocalVariables|GetReturn) (LocalVariables|GetAnalyzedPosition))
              (LocalVariables|SetbHit true))))))
    (for _array_element_2 _innactiveunits
      (Utilities|IsValid _array_element_2
        (:Is%20Valid
          (if (!= (Default|GetPosition _array_element_2) StartPosition)
            (bind _output_get_2 (LocalVariables|SetAnalyzedPosition (Default|GetPosition _array_element_2)))
            (if (Utilities|Array|ContainsItem Positions _output_get_2)
              (Utilities|Array|AddUnique (LocalVariables|GetReturn) (LocalVariables|GetAnalyzedPosition))
              (LocalVariables|SetbHit true))))))
    (return (LocalVariables|GetbHit) (LocalVariables|GetReturn))
    (else
      (return false (Utilities|Array|MakeArray (Utilities|Struct|MakeIntPoint -999 -999))))))

(fn ClosestPosition
  (params (OriginPosition :type Int%20Point%20Structure) (ReferencePosition :type Int%20Point%20Structure%20%28by%20ref%29))
  (LocalVariables|SetOriginLocation (.worldlocation (.TileData (Default|GetTileData (Variables|Default|GetGrid)))))
  (LocalVariables|SetReferenceLocation (.worldlocation (.TileData (Default|GetTileData (Variables|Default|GetGrid)))))
  (bind _output_get (LocalVariables|SetDirectionalVector (* (Math|Vector|Normalize (- (LocalVariables|GetReferenceLocation) (LocalVariables|GetOriginLocation)) 0.01) (LocalVariables|GetHexagonSizeFactor))))
  (return (not (Utilities|IsValid (Utilities|Struct|BreakGridTileOccupancy (.occupancy (.TileData (Default|GetTileData (Variables|Default|GetGrid) "")))))) ""))

(fn SetSpellEffect
  (params (SpellEffectType :type E_SpellEffectHandler%20Enum :default "NewEnumerator2"))
  (Variables|Default|SetSpellEffectType SpellEffectType))