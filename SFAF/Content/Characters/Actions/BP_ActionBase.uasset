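; BP_ActionBase is the base actor for character actions that operate on BP_Grid tiles.
; On BeginPlay it retries finding the grid every 0.2 seconds, then signals that it is ready.
; ExecuteAction returns tile data for two positions, with success based on the first, or fails and re-fetches an invalid grid.
; It also stores its owning pawn and controller, setting the controller as owner, and can destroy itself.
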(event EventBeginPlay
  (bind _returnvalue (Actor|GetActorOfClass "/Game/Ground/Terrain/BP_Grid.BP_Grid_C" :!label _label))
  (bind _output_get (Variables|Default|SetGrid _returnvalue))
  (Utilities|IsValid _output_get
    (:Is%20Valid
      (Default|CallReadytoUse)
      (Class|ActionBase|SetReady true))
    (:Is%20Not%20Valid
      (Utilities|FlowControl|Delay 0.2)
      (goto _label))))

(event Collision|EventActorBeginOverlap
  (params (OtherActor :type Actor%20Object%20Reference)))

(fn ConstructionScript)

(fn ExecuteAction
  (params (Position%201 :type Int%20Point%20Structure) (bHitResult :type Boolean) (Position%202 :type Int%20Point%20Structure))
  (bind _gridtilestaticdata (Utilities|Struct|MakeGridTileStaticData "0.000000,0.000000,0.000000" -1 "(GameplayTags=)" "(OccupyingUnit=None)"))
  (Utilities|IsValid (Variables|Default|GetGrid)
    (:Is%20Valid
      (return (.Success (Default|GetTileData (Variables|Default|GetGrid) Position%201)) (.TileData (Default|GetTileData (Variables|Default|GetGrid) Position%201)) (.TileData (Default|GetTileData (Variables|Default|GetGrid) Position%202))))
    (:Is%20Not%20Valid
      (bind _returnvalue (Actor|GetActorOfClass "/Game/Ground/Terrain/BP_Grid.BP_Grid_C"))
      (Variables|Default|SetGrid _returnvalue)
      (return false _gridtilestaticdata _gridtilestaticdata))))

(fn DestroyAction
  (Development|PrintString "Being destroyed")
  (Actor|DestroyActor))

(fn SetOwningEntities
  (params (Pawn :type Pawn%20Object%20Reference) (Controller :type Controller%20Object%20Reference))
  (Variables|Components|SetPawn Pawn)
  (bind _output_get (Variables|Default|SetController Controller))
  (Actor|SetOwner _output_get))