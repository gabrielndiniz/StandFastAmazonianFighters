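; BP_ActionHoverTile is a grid action that marks the tile at the hovered position with a highlight plane.
; ExecuteAction runs the parent action, then moves HoverPlane to the returned tile's world location, or hides it on failure.
; SetTileStatus can move the grid's Hovered state, checking BP_ActionSelectTile's selection.
; ExecuteAction ANDs its hit flag with false, so that call only ever takes the clearing branch.
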(event EventBeginPlay
  (|CallParentFunction)
  (Utilities|FlowControl|Delay 0.1)
  (bind _returnvalue (Actor|GetActorOfClass "/Game/Characters/Actions/StandardPlayActions/BP_ActionSelectTile.BP_ActionSelectTile_C"))
  (Variables|Default|SetSelect _returnvalue))

(event Collision|EventActorBeginOverlap
  (params (OtherActor :type Actor%20Object%20Reference))
  (|CallParentFunction OtherActor) ; This node is disabled and will not be called.\nDrag off pins to build functionality.
)

(event EventTick
  (params (DeltaSeconds :type Float%20%28single-precision%29))
  (|CallParentFunction DeltaSeconds) ; This node is disabled and will not be called.\nDrag off pins to build functionality.
)

(fn ConstructionScript
  (|CallParentFunction))

(fn SetHoverPlaneLocation
  (params (NewLocation :type Vector) (bHide :type Boolean))
  (bind _hoverplane (Variables|Default|GetHoverPlane))
  (if (Utilities|Operators|NotEqual(!=) NewLocation (Transformation|GetWorldLocation (Variables|Default|GetHoverPlane)) 0.01)
    (if bHide
      (Rendering|SetVisibility _hoverplane false false)
      (else
        (Transformation|SetWorldLocation _hoverplane NewLocation false false)
        (if (not (Rendering|IsVisible (Variables|Default|GetHoverPlane)))
          (Rendering|SetVisibility (Variables|Default|GetHoverPlane) true true))))))

(fn ExecuteAction
  (params (Position%201 :type Int%20Point%20Structure) (bHitResult :type Boolean) (Position%202 :type Int%20Point%20Structure))
  (bind (_success _tiledata1) (|CallParentFunction Position%201 bHitResult Position%202))
  (LocalVariables|SetContinue _success)
  (Utilities|IsValid (Variables|Default|GetGrid)
    (:Is%20Valid
      (CallFunction|SetTileStatus (Math|Boolean|ANDBoolean bHitResult (LocalVariables|GetContinue) false) Position%201)
      (if (LocalVariables|GetContinue)
        (LocalVariables|SetData _tiledata1)
        (CallFunction|SetHoverPlaneLocation (.worldlocation (LocalVariables|GetData)) false)
        (return (LocalVariables|GetContinue) (LocalVariables|GetData) "")
        (else
          (CallFunction|SetHoverPlaneLocation "0.000000,0.000000,9999.000000" true)
          (return (LocalVariables|GetContinue) (LocalVariables|GetData) ""))))
    (:Is%20Not%20Valid
      (return false "" ""))))

(fn SetTileStatus
  (params (bHitResult :type Boolean) (Position :type Int%20Point%20Structure))
  (if bHitResult
    (LocalVariables|SetCurrentPosition Position)
    (Utilities|IsValid (Variables|Default|GetSelect)
      (:Is%20Valid
        _)
      (:Is%20Not%20Valid
        (bind _returnvalue (Actor|GetActorOfClass "/Game/Characters/Actions/StandardPlayActions/BP_ActionSelectTile.BP_ActionSelectTile_C"))
        (Variables|Default|SetSelect _returnvalue)))
    (if (!= (Default|GetSelectedTile (Variables|Default|GetSelect)) (LocalVariables|GetCurrentPosition))
      (if (!= (LocalVariables|GetCurrentPosition) (Variables|Default|GetHoveredGridPosition))
        (Default|RemoveStateTile (Variables|Default|GetGrid) (Variables|Default|GetHoveredGridPosition) "Hovered")
        (Variables|Default|SetHoveredGridPosition (LocalVariables|GetCurrentPosition))
        (Default|AddStateTile (Variables|Default|GetGrid) (LocalVariables|GetCurrentPosition) "Hovered"))
      (elif (!= (Default|GetSelectedTile (Variables|Default|GetSelect)) (Variables|Default|GetHoveredGridPosition))
        (Default|RemoveStateTile (Variables|Default|GetGrid) (Variables|Default|GetHoveredGridPosition) "Hovered")
        (bind _output_get (Variables|Default|SetHoveredGridPosition (Default|GetSelectedTile (Variables|Default|GetSelect))))
        (Default|AddStateTile (Variables|Default|GetGrid) _output_get "Hovered")))
    (elif (!= (Variables|Default|GetHoveredGridPosition) (Utilities|Struct|MakeIntPoint 9999 9999))
      (Default|AddStateTile (Variables|Default|GetGrid) (Variables|Default|GetHoveredGridPosition) "None")
      (Variables|Default|SetHoveredGridPosition (Utilities|Struct|MakeIntPoint 9999 9999)))))