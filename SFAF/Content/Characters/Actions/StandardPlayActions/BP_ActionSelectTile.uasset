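; Tile-selection action that marks the chosen grid tile with a cyan hexagon and can display a set of reachable tiles.
; When the parent action succeeds, ExecuteAction moves the hexagon, transfers the grid's Selected state and rebuilds the reachable markers.
; Reachables are supplied through a setter and drawn as toggleable instanced meshes raised slightly above each tile.
; ChangeHexagonColor pulses the hexagon's emission and opacity through material parameters, but nothing here calls it.
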(event EventBeginPlay
  (|CallParentFunction) ; This node is disabled and will not be called.\nDrag off pins to build functionality.
)

(event Collision|EventActorBeginOverlap
  (params (OtherActor :type Actor%20Object%20Reference))
  (|CallParentFunction OtherActor) ; This node is disabled and will not be called.\nDrag off pins to build functionality.
)

(event EventTick
  (params (DeltaSeconds :type Float%20%28single-precision%29))
  (|CallParentFunction DeltaSeconds) ; This node is disabled and will not be called.\nDrag off pins to build functionality.
)

(fn ConstructionScript
  (bind _hexagon (Variables|Default|GetHexagon))
  (|CallParentFunction)
  (Rendering|Material|SetVectorParameterValueonMaterials _hexagon "Color" (Math|Conversions|ToVector(LinearColor) (Math|Color|MakeColor 0.07 0.8 0.9)))
  (Rendering|Material|SetScalarParameterValueonMaterials _hexagon "MultiplierForEmissionAndOpacity" (Variables|Default|GetBrightMultiply))
  (Rendering|Material|SetScalarParameterValueonMaterials _hexagon "AddAfterMultiplier" (Variables|Default|GetBrightAdder)))

(fn SetHexagonLocation
  (params (NewLocation :type Vector))
  (Transformation|SetWorldLocation (Variables|Default|GetHexagon) NewLocation false false))

(fn ExecuteAction
  (params (Position%201 :type Int%20Point%20Structure) (bHitResult :type Boolean) (Position%202 :type Int%20Point%20Structure))
  (bind (_success _tiledata1) (|CallParentFunction Position%201 bHitResult Position%202))
  (bind _output_get (LocalVariables|SetContinue _success))
  (if _output_get
    (bind _output_get_2 (LocalVariables|SetData _tiledata1))
    (CallFunction|SetHexagonLocation (.worldlocation _output_get_2))
    (CallFunction|SetTileStatus Position%201)
    (CallFunction|ShowReachables))
  (return (LocalVariables|GetContinue) (LocalVariables|GetData) ""))

(fn ChangeHexagonColor
  (bind _hexagon (Variables|Default|GetHexagon))
  (Rendering|Material|SetScalarParameterValueonMaterials _hexagon "MultiplierForEmissionAndOpacity" (Variables|Default|GetBrightMultiply))
  (Rendering|Material|SetScalarParameterValueonMaterials _hexagon "AddAfterMultiplier" (Variables|Default|GetBrightAdder))
  (if (or (>= (Variables|Default|GetBrightAdder) 1.0) (<= (Variables|Default|GetBrightAdder) 0.0))
    (Variables|Default|SetChangeColorSpeed (* (Variables|Default|GetChangeColorSpeed) -1.0)))
  (Variables|Default|SetBrightAdder (+ (* (Variables|Default|GetChangeColorSpeed) (Utilities|Time|GetWorldDeltaSeconds)) (Variables|Default|GetBrightAdder)))
  (Variables|Default|SetBrightMultiply (+ (* (* (Variables|Default|GetChangeColorSpeed) (Utilities|Time|GetWorldDeltaSeconds)) -2.0) (Variables|Default|GetBrightMultiply))))

(fn GetSelectedTile
  (return (Variables|Default|GetSelectedGridPositon)))

(fn SetTileStatus
  (params (Position :type Int%20Point%20Structure))
  (if (!= Position (Variables|Default|GetSelectedGridPositon))
    (Default|RemoveStateTile :self (Variables|Default|GetGrid) :Tile%20State "Selected")
    (Variables|Default|SetSelectedGridPositon Position)
    (Default|AddStateTile :self (Variables|Default|GetGrid) :GridTileState "Selected")))

(fn SetReachables
  (params (Reachables :type Array%20of%20Int%20Point%20Structures))
  (Variables|Default|SetReachables Reachables))

(fn ShowReachables
  (bind _grid (Variables|Default|GetGrid))
  (bind _tiledata (Default|GetTileData _grid ""))
  (bind (_x _y _z) (Math|Vector|BreakVector (.worldlocation _tiledata)))
  (Components|InstancedStaticMesh|ClearInstances (Variables|Default|GetInstancedStaticMeshReachables))
  (if (Variables|Default|GetbShowReachables)
    (for _array_element (Variables|Default|GetReachables)
      (Components|InstancedStaticMesh|AddInstance (Variables|Default|GetInstancedStaticMeshReachables) (Math|Transform|MakeTransform (Math|Vector|MakeVector _x _y (+ _z 4.0)) "0, 0, 0" "1.000000,1.000000,1.000000") true))))

(fn SetShowReachables
  (params (bShowReachables :type Boolean))
  (Variables|Default|SetbShowReachables bShowReachables)
  (CallFunction|ShowReachables))

(fn GetReachables
  (return (Variables|Default|GetReachables)))