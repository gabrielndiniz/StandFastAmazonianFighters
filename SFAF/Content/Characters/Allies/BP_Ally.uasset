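; BP_Ally is an allied unit Blueprint that adds skeletal-mesh animation behavior to a parent unit class.
; Its movement, idle, attack, damage and death functions message the Anim Instance with an animation state enum, with damage and death also running parent logic.
; The attack event triggers the attack animation.
; The hide event calls its parent, waits a few seconds, then moves the mesh far off-world instead of destroying it.
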(event EventBeginPlay
  (|CallParentFunction) ; This node is disabled and will not be called.\nDrag off pins to build functionality.
)

(event Collision|EventActorBeginOverlap
  (params (OtherActor :type Actor%20Object%20Reference))
  (|CallParentFunction OtherActor) ; This node is disabled and will not be called.\nDrag off pins to build functionality.
)

(event EventTick
  (params (DeltaSeconds :type Float%20%28single-precision%29))
  (|CallParentFunction DeltaSeconds) ; This node is disabled and will not be called.\nDrag off pins to build functionality.
)

(event EventEventHideUnitAfterFewSeconds
  (|CallParentFunction)
  (Utilities|FlowControl|Delay 5.0)
  (Transformation|SetRelativeLocation (Variables|Default|GetSkeletalMesh) "-99999.000000,-99999.000000,-99999.000000" false false))

(event EventEventAttack
  (params (Target%20Position :type Int%20Point%20Structure))
  (CallFunction|AttackAnimation))

(fn ConstructionScript
  (|CallParentFunction))

(fn MovingAnimation
  (Class|BPIUnitAnimation|SetUnitAnimationState(Message) (Components|SkeletalMesh|GetAnimInstance (Variables|Default|GetSkeletalMesh)) "NewEnumerator1"))

(fn BacktoIdle
  (Class|BPIUnitAnimation|SetUnitAnimationState(Message) (Components|SkeletalMesh|GetAnimInstance (Variables|Default|GetSkeletalMesh)) "NewEnumerator0"))

(fn AttackAnimation
  (Class|BPIUnitAnimation|SetUnitAnimationState(Message) (Components|SkeletalMesh|GetAnimInstance (Variables|Default|GetSkeletalMesh)) "NewEnumerator2"))

(fn UnitDamaged
  (|CallParentFunction)
  (Class|BPIUnitAnimation|SetUnitAnimationState(Message) (Components|SkeletalMesh|GetAnimInstance (Variables|Default|GetSkeletalMesh)) "NewEnumerator3"))

(fn UnitDied
  (|CallParentFunction)
  (Class|BPIUnitAnimation|SetUnitAnimationState(Message) (Components|SkeletalMesh|GetAnimInstance (Variables|Default|GetSkeletalMesh)) "NewEnumerator4"))