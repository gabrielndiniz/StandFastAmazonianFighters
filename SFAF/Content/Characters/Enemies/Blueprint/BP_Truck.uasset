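; BP_Truck is an enemy character whose attack lunges its static mesh along the actor's forward vector.
; A DoOnce-guarded timeline offsets the mesh from the actor's location by curve value times Velocity, without sweeping or moving the actor itself.
; When the timeline finishes, the mesh snaps back to the relative location cached on BeginPlay or reset, and the guard reopens.
; Construction and damage handling only call the parent.
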(event EventOnReset
  (|CallParentFunction)
  (Variables|Default|SetInitial%20Location (Variables|/Script/Engine.SceneComponent|GetRelativeLocation (Variables|Default|GetStaticMesh))))

(event EventEventAttack
  (params (Target%20Position :type Int%20Point%20Structure))
  (|CallParentFunction Target%20Position)
  (Utilities|FlowControl|DoOnce false :!label _label
    (:Completed
      (bind _floatcurve (Timeline|Timeline PlayFromStart)
        (:Update
          (Transformation|SetWorldLocation (Variables|Default|GetStaticMesh) (+ (* _floatcurve (Transformation|GetActorForwardVector) (Variables|Default|GetVelocity)) (Transformation|GetActorLocation)) false false))
        (:Finished
          (Utilities|FlowControl|Sequence
            (:then_0
              (Transformation|SetRelativeLocation (Variables|Default|GetStaticMesh) (Variables|Default|GetInitial%20Location) false false))
            (:then_1
              (goto _label Reset))))))))

(event EventBeginPlay
  (|CallParentFunction)
  (Variables|Default|SetInitial%20Location (Variables|/Script/Engine.SceneComponent|GetRelativeLocation (Variables|Default|GetStaticMesh))))

(fn ConstructionScript
  (|CallParentFunction))

(fn UnitDamaged
  (|CallParentFunction))