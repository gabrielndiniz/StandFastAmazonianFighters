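; BP_Harvester is an enemy unit whose attack procedurally swings a bladed arm.
; On BeginPlay and reset, it sets the Joint, Wrist and Blades components to their initial yaw, roll and yaw rotations.
; An attack plays a timeline that drives those rotations, with a DoOnce blocking retriggers until it finishes and restores the initial pose.
; Damage, death and hiding defer to the parent class.
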(event EventBeginPlay
  (|CallParentFunction)
  (Transformation|SetRelativeRotation (Variables|Default|GetJoint) (Math|Rotator|MakeRotator 0.0 0.0 (Variables|Default|GetInitialJointRotation)) false false)
  (Transformation|SetRelativeRotation (Variables|Default|GetWrist) (Math|Rotator|MakeRotator (Variables|Default|GetInitialWristRotation) 0.0 0.0) false false)
  (Transformation|SetRelativeRotation (Variables|Default|GetBlades) (Math|Rotator|MakeRotator 0.0 0.0 (Variables|Default|GetInitialBladesRotation)) false false))

(event EventEventAttack
  (params (Target%20Position :type Int%20Point%20Structure))
  (|CallParentFunction Target%20Position)
  (Utilities|FlowControl|DoOnce false :!label _label
    (:Completed
      (bind (_direction _jointrotation _wristrotation _bladesrotation) (Timeline|Timeline PlayFromStart)
        (:Update
          (Transformation|SetRelativeRotation (Variables|Default|GetJoint) (Math|Rotator|MakeRotator 0.0 0.0 _jointrotation) false false)
          (Transformation|SetRelativeRotation (Variables|Default|GetWrist) (Math|Rotator|MakeRotator _wristrotation 0.0 0.0) false false)
          (Transformation|SetRelativeRotation (Variables|Default|GetBlades) (Math|Rotator|MakeRotator 0.0 0.0 _bladesrotation) false false))
        (:Finished
          (Utilities|FlowControl|Sequence
            (:then_0
              (Transformation|SetRelativeRotation (Variables|Default|GetJoint) (Math|Rotator|MakeRotator 0.0 0.0 (Variables|Default|GetInitialJointRotation)) false false)
              (Transformation|SetRelativeRotation (Variables|Default|GetWrist) (Math|Rotator|MakeRotator (Variables|Default|GetInitialWristRotation) 0.0 0.0) false false)
              (Transformation|SetRelativeRotation (Variables|Default|GetBlades) (Math|Rotator|MakeRotator 0.0 0.0 (Variables|Default|GetInitialBladesRotation)) false false))
            (:then_1
              (goto _label Reset))))))))

(event EventOnReset
  (|CallParentFunction)
  (Transformation|SetRelativeRotation (Variables|Default|GetJoint) (Math|Rotator|MakeRotator 0.0 0.0 (Variables|Default|GetInitialJointRotation)) false false)
  (Transformation|SetRelativeRotation (Variables|Default|GetWrist) (Math|Rotator|MakeRotator (Variables|Default|GetInitialWristRotation) 0.0 0.0) false false)
  (Transformation|SetRelativeRotation (Variables|Default|GetBlades) (Math|Rotator|MakeRotator 0.0 0.0 (Variables|Default|GetInitialBladesRotation)) false false))

(event EventEventHideUnitAfterFewSeconds
  (|CallParentFunction))

(fn ConstructionScript
  (|CallParentFunction))

(fn UnitDamaged
  (|CallParentFunction))

(fn UnitDied
  (|CallParentFunction))