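; Wheeled enemy unit that animates its wheels while moving and bursts apart with physics on death.
; InitiateWheels gathers physics constraints under StaticMesh, their child wheel meshes and bounds-derived sizes.
; While MovingAnimation's flag is set, Tick rolls the constraints by speed and wheel size until BackToIdle clears it.
; UnitDied activates Death, frees constraints and impulses the parts outward; the hide event later moves body and wheels far away.
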(event EventEventHideUnitAfterFewSeconds
  (bind _staticmesh (Variables|Default|GetStaticMesh))
  (|CallParentFunction)
  (Utilities|FlowControl|Delay 5.0)
  (Utilities|IsValid _staticmesh
    (:Is%20Valid
      (Transformation|SetRelativeLocation _staticmesh "-99999.000000,-99999.000000,-99999.000000" false false)
      (for _array_element (Variables|Default|GetWheels)
        (Utilities|IsValid _array_element
          (:Is%20Valid
            (Transformation|SetRelativeLocation _array_element "-99999.000000,-99999.000000,-99999.000000" false false)))))))

(event EventTick
  (params (DeltaSeconds :type Float%20%28single-precision%29))
  (|CallParentFunction DeltaSeconds)
  (if (Variables|Default|GetbSpinWheels)
    (CallFunction|SpinWheels)))

(event EventBeginPlay
  (|CallParentFunction)
  (CallFunction|InitiateWheels))

(event EventOnReset
  (|CallParentFunction)
  (CallFunction|InitiateWheels))

(fn ConstructionScript
  (|CallParentFunction))

(fn SpinWheels
  (bind _constrains (Variables|Default|GetConstrains))
  (bind _returnvalue (Utilities|Array|LastIndex _constrains))
  (if (not (Utilities|Array|IsEmpty (Variables|Default|GetWheels)))
    (if (Utilities|Array|IsEmpty (Variables|Default|GetConstrains))
      (CallFunction|InitiateWheels))
    (if (and (== (Utilities|Array|LastIndex (Variables|Default|GetWheels)) _returnvalue) (== _returnvalue (Utilities|Array|LastIndex (Variables|Default|GetWheelsSize))))
      _
      (else
        (CallFunction|InitiateWheels)))
    (for (_array_element _array_index) (Variables|Default|GetConstrains)
      (Utilities|IsValid _array_element
        (:Is%20Valid
          (Transformation|SetRelativeRotation _array_element (Math|Rotator|MakeRotator (+ (* (* (LocalVariables|GetSpeedAdjustment) (Variables|Default|GetMoveSpeed)) (/ (Math|Float|MultiplybyPi (Utilities|Array|Get(acopy) (Variables|Default|GetWheelsSize) _array_index)) 3.6e+02) (Utilities|Time|GetWorldDeltaSeconds)) (.roll (Variables|/Script/Engine.SceneComponent|GetRelativeRotation _array_element))) (.pitch (Variables|/Script/Engine.SceneComponent|GetRelativeRotation _array_element)) (.yaw (Variables|/Script/Engine.SceneComponent|GetRelativeRotation _array_element))) false false))))
    (return)))

(fn MovingAnimation
  (Variables|Default|SetbSpinWheels true))

(fn InitiateWheels
  (if (not (Utilities|Array|IsEmpty (Variables|Default|GetWheels)))
    (Utilities|IsValid (Variables|Default|GetStaticMesh)
      (:Is%20Valid
        (for _array_element (Components|GetChildrenComponents (Variables|Default|GetStaticMesh) false)
          (Utilities|IsValid _array_element
            (:Is%20Valid
              (bind _asphysics_constraint_component (Utilities|Casting|CastToPhysicsConstraintComponent _array_element))
              (Utilities|Array|Add (Variables|Default|GetConstrains) _asphysics_constraint_component)
              (bind _asstatic_mesh_component (Utilities|Casting|CastToStaticMeshComponent (Components|GetChildComponent _asphysics_constraint_component 0)))
              (Utilities|IsValid _asstatic_mesh_component
                (:Is%20Valid
                  (Utilities|Array|Add (Variables|Default|GetWheels) _asstatic_mesh_component)
                  (Utilities|Array|Add (Variables|Default|GetWheelsSize) (* (Math|Vector|DotProduct (.Max (Components|StaticMesh|GetLocalBounds _asstatic_mesh_component)) (Math|Vector|GetUpVector _asstatic_mesh_component)) (Math|Vector|DotProduct (Math|Vector|GetUpVector _asstatic_mesh_component) (Transformation|GetWorldScale _asstatic_mesh_component)))))))))))))

(fn BacktoIdle
  (Variables|Default|SetbSpinWheels false))

(fn UnitDied
  (bind _staticmesh (Variables|Default|GetStaticMesh))
  (bind _staticmesh_2 (Variables|Default|GetStaticMesh))
  (|CallParentFunction)
  (Components|Activation|Activate (Variables|Default|GetDeath) true)
  (Utilities|IsValid _staticmesh
    (:Is%20Valid
      (for _array_element (Components|GetChildrenComponents _staticmesh true)
        (Utilities|IsValid _array_element
          (:Is%20Valid
            (bind _asphysics_constraint_component (Utilities|Casting|CastToPhysicsConstraintComponent _array_element)
              (:then
                (Class|PhysicsConstraintComponent|SetAngularSwing1Limit _asphysics_constraint_component "ACM_Free" 0.0)
                (Class|PhysicsConstraintComponent|SetAngularSwing2Limit _asphysics_constraint_component "ACM_Free" 0.0)
                (Class|PhysicsConstraintComponent|SetAngularTwistLimit _asphysics_constraint_component "ACM_Free" 0.0)
                (Class|PhysicsConstraintComponent|SetLinearXLimit _asphysics_constraint_component "LCM_Free" 0.0)
                (Class|PhysicsConstraintComponent|SetLinearYLimit _asphysics_constraint_component "LCM_Free" 0.0)
                (Class|PhysicsConstraintComponent|SetLinearZLimit _asphysics_constraint_component "LCM_Free" 0.0))
              (:CastFailed
                (bind _asstatic_mesh_component (Utilities|Casting|CastToStaticMeshComponent _array_element))
                (Physics|SetSimulatePhysics _asstatic_mesh_component true)
                (Physics|SetEnableGravity _asstatic_mesh_component true)
                (Physics|AddImpulse _asstatic_mesh_component (* (Variables|/Script/Engine.SceneComponent|GetRelativeLocation _asstatic_mesh_component) (LocalVariables|GetImpulseOnComponents)) "None" true)
                (Collision|SetCollisionResponsetoChannel _asstatic_mesh_component "ECC_GameTraceChannel1" "ECR_Block"))))))
      (Utilities|IsValid _staticmesh_2
        (:Is%20Valid
          (Physics|SetSimulatePhysics _staticmesh_2 true)
          (Physics|SetEnableGravity _staticmesh_2 true)
          (Collision|SetCollisionResponsetoChannel _staticmesh_2 "ECC_GameTraceChannel1" "ECR_Block")
          (Physics|AddImpulse _staticmesh_2 (* (Variables|/Script/Engine.SceneComponent|GetRelativeLocation _staticmesh_2) (LocalVariables|GetImpulseOnMainBody)) "None" true))))))

(fn UnitDamaged
  (|CallParentFunction))