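; BP_GridDataComponent holds the ground grid's spawn and shape settings and resolves the assets for its shape.
; SetShapeData stores spawn location, tile size and count, the Color enum and spawn-mode options.
; GetShapeData uses Color's name as the DT_GridShapeData row key, returning mesh size, solid and plane assets, material instances and tile count.
; A missing row only prints an error.
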(fn GetShapeData
  (bind _returnvalue (Utilities|GetDataTableRow "/Game/Ground/Enum/DT_GridShapeData.DT_GridShapeData" (Utilities|String|StringToName (Utilities|String|EnumtoString (Variables|Default|GetColor))))
    (:then
      (return (.MeshSize (Utilities|Struct|BreakST_GridShapeData _returnvalue)) (.Solid (Utilities|Struct|BreakST_GridShapeData _returnvalue)) (.SolidWithMoldureMaterialInstance (Utilities|Struct|BreakST_GridShapeData _returnvalue)) (.Plane (Utilities|Struct|BreakST_GridShapeData _returnvalue)) (.PlaneMaterialInstance (Utilities|Struct|BreakST_GridShapeData _returnvalue)) (.PlaneBorderMaterialInstance (Utilities|Struct|BreakST_GridShapeData _returnvalue)) (.UniversalMaterialInstance (Utilities|Struct|BreakST_GridShapeData _returnvalue)) (Variables|Default|GetGrid%20Tile%20Count)))
    (:RowNotFound
      (Development|PrintString "Error #X9&: Row not found in BP_Grid" true true "(R=1.000000,G=0.000000,B=0.046707,A=1.000000)"))))

(fn SetShapeData
  (params (Initial%20Spawn%20Location :type Vector) (Grid%20Tile%20Size :type Vector) (Grid%20Tile%20Count :type Int%20Point%20Structure) (Color :type E_GridShape%20Enum :default "NewEnumerator0") (Spawn%20Around%20Given%20Location :type Boolean) (Spawn%20On%20Environment :type Boolean))
  (Variables|Default|SetInitial%20Spawn%20Location Initial%20Spawn%20Location)
  (Variables|Default|SetGrid%20Tile%20Size Grid%20Tile%20Size)
  (Variables|Default|SetGrid%20Tile%20Count Grid%20Tile%20Count)
  (Variables|Default|SetColor Color)
  (Variables|Default|SetbSpawn%20Around%20Given%20Location Spawn%20Around%20Given%20Location)
  (Variables|Default|SetbSpawn%20on%20Environment Spawn%20On%20Environment))