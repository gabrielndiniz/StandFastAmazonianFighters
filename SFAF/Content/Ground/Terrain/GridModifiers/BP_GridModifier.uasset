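; Placeable hex-grid modifier actor that marks a tile's type (normal, obstacle, cost multiplier, flying-only) and exposes that type and a use-for-height flag.
; Construction hands the level's BP_Grid to its GridSnapComponent and styles the hexagon preview mesh by type through material and colour parameters.
; Obstacle tiles block GameTraceChannel7, set at construction and again from tile tags at BeginPlay.
; The preview hides at BeginPlay and shows only while tactical mode is on.
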(event EventBeginPlay
  (Development|SetHiddeninGame (Variables|Default|GetPreviewMesh) true false)
  (if (GameplayTags|HasTag (Class|GridModifier|GetTileTags) "(TagName=\"Grid.Type.Obstacle\")")
    (Collision|SetCollisionResponsetoChannel (Variables|Default|GetPreviewMesh) "ECC_GameTraceChannel7" "ECR_Block")))

(event Collision|EventActorBeginOverlap
  (params (OtherActor :type Actor%20Object%20Reference)))

(event EventTick
  (params (DeltaSeconds :type Float%20%28single-precision%29)))

(fn ConstructionScript
  (bind _type (Variables|Default|GetType))
  (bind _returnvalue (Utilities|Select :Index _type :NewEnumerator0 "(R=0.000000,G=1.000000,B=0.000000,A=1.000000)" :NewEnumerator1 "(R=0.000000,G=0.000000,B=0.000000,A=1.000000)" :NewEnumerator2 "(R=1.000000,G=0.000000,B=0.839263,A=1.000000)" :NewEnumerator3 "(R=0.132568,G=1.000000,B=0.000000,A=1.000000)" :NewEnumerator4 "(R=1.000000,G=0.025978,B=0.000000,A=1.000000)" :NewEnumerator5 "(R=0.000000,G=0.029868,B=1.000000,A=1.000000)"))
  (bind _returnvalue_2 (Math|Conversions|ToVector(LinearColor) _returnvalue))
  (bind _returnvalue_3 (Actor|GetActorOfClass "/Game/Ground/Terrain/BP_Grid.BP_Grid_C"))
  (Class|GridSnapComponent|SetGrid (Variables|Default|GetGridSnapComponent) _returnvalue_3)
  (Components|StaticMesh|SetStaticMesh (Variables|Default|GetPreviewMesh) "/Game/Ground/Meshes/Traditional/Meshes/SM_HexagonZ100.SM_HexagonZ100")
  (Rendering|Material|SetMaterial (Variables|Default|GetPreviewMesh) 0 (Utilities|Select :Index _type :NewEnumerator0 "/Game/Ground/Meshes/Traditional/Material/Z150/MI_HexagonZ150_WithMoldure_Green.MI_HexagonZ150_WithMoldure_Green" :NewEnumerator1 "/Game/Ground/Meshes/Traditional/Material/Z150/M_HexagonZ150_WithMoldure.M_HexagonZ150_WithMoldure" :NewEnumerator2 "/Game/Ground/Meshes/Traditional/Material/Z150/MI_HexagonZ150_WithMoldure_Black.MI_HexagonZ150_WithMoldure_Black" :NewEnumerator3 "/Game/Ground/Meshes/Traditional/Material/Z150/MI_HexagonZ150_WithMoldure_Green.MI_HexagonZ150_WithMoldure_Green" :NewEnumerator4 "/Game/Ground/Meshes/Traditional/Material/Z150/MI_HexagonZ150_WithMoldure_Red.MI_HexagonZ150_WithMoldure_Red" :NewEnumerator5 "/Game/Ground/Meshes/Traditional/Material/Z150/MI_HexagonZ150_WithMoldure_Blue.MI_HexagonZ150_WithMoldure_Blue"))
  (Rendering|Material|SetVectorParameterValueonMaterials (Variables|Default|GetPreviewMesh) "InternalColor" _returnvalue_2)
  (Rendering|Material|SetVectorParameterValueonMaterials (Variables|Default|GetPreviewMesh) "ExternalColor" (* _returnvalue_2 0.4))
  (Collision|SetCollisionResponsetoChannel (Variables|Default|GetPreviewMesh) "ECC_GameTraceChannel3" "ECR_Ignore")
  (Development|SetHiddeninGame (Variables|Default|GetPreviewMesh) false false)
  (if (== (Class|GridModifier|GetTileModificationTag) "(TagName=\"Grid.Type.Obstacle\")")
    (Collision|SetCollisionResponsetoChannel (Variables|Default|GetPreviewMesh) "ECC_GameTraceChannel7" "ECR_Block")))

(fn GetModificationType
  (return (Class|GridModifier|GetTileModificationTag)))

(fn GetUseforHeight
  (return (Variables|Default|GetbUseForHeight)))

(fn SetTacticalMode
  (params (Tactical%20Mode :type Boolean))
  (Development|SetHiddeninGame (Variables|Default|GetPreviewMesh) (not Tactical%20Mode) false))