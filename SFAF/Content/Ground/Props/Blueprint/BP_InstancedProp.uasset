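; BP_InstancedProp is a ground prop with a preview mesh and a component for snapping to the level grid.
; Its construction script sets the preview mesh to overlap a custom trace channel, then finds the BP_Grid actor and passes it to the snap component.
; SetColor has an empty entry: its disconnected logic would tint the mesh red or green by tile diagonal in three shades, but never runs.
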(event EventBeginPlay)

(fn ConstructionScript
  (Collision|SetCollisionResponsetoChannel (Variables|Default|GetPreviewMesh) "ECC_GameTraceChannel3" "ECR_Overlap")
  (bind _returnvalue (Actor|GetActorOfClass "/Game/Ground/Terrain/BP_Grid.BP_Grid_C"))
  (bind _asgrid_type (Utilities|Casting|CastToGridType _returnvalue)
    (:then
      (Class|GridSnapComponent|SetGrid (Variables|Default|GetGridSnapComponent) _asgrid_type))
    (:CastFailed
      (Development|PrintString "cast failed 1"))))

(fn SetColor
  (params (TurnRedOnYValue :type Integer) (XAdjust :type Float%20%28double-precision%29)))