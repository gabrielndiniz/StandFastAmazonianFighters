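; BP_RandomTree is a tree prop that randomizes its look in the construction script.
; It picks one of three meshes and one of three materials, creating a dynamic material instance from the latter.
; Weighted random scalars vary the new leaves, old leaves and wood parameters.
; The mesh also gets a random yaw and a weighted random height scale, with unseeded randomness rerolling whenever construction reruns.
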(fn ConstructionScript
  (bind _weightofrandomscale (Variables|Default|GetWeightOfRandomScale))
  (bind _staticmesh (Variables|Default|GetStaticMesh))
  (bind _weightofrandomcolor (Variables|Default|GetWeightOfRandomColor))
  (bind _weightofrandomcolor_2 (Variables|Default|GetWeightOfRandomColor))
  (bind _weightofrandomcolor_3 (Variables|Default|GetWeightOfRandomColor))
  (Components|StaticMesh|SetStaticMesh _staticmesh (Utilities|Array|Get(acopy) (Variables|Default|GetTree%20Meshes) (Math|Random|RandomInteger 3)))
  (bind _returnvalue (Rendering|Material|CreateDynamicMaterialInstance _staticmesh 0 (Utilities|Array|Get(acopy) (Variables|Default|GetTree%20Materials) (Math|Random|RandomInteger 3)) "None" :!class /Script/Engine.PrimitiveComponent))
  (bind _output_get (Variables|Default|SetMaterial _returnvalue))
  (Rendering|Material|SetScalarParameterValue _output_get "NewLeaves" (+ (* (Math|Random|RandomFloat) _weightofrandomcolor) (- 1.0 _weightofrandomcolor)) :!class /Script/Engine.MaterialInstanceDynamic)
  (Rendering|Material|SetScalarParameterValue _output_get "OldLeaves" (+ (* (Math|Random|RandomFloat) _weightofrandomcolor_2) (- 1.0 _weightofrandomcolor_2)) :!class /Script/Engine.MaterialInstanceDynamic)
  (Rendering|Material|SetScalarParameterValue _output_get "Wood" (+ (* (Math|Random|RandomFloat) _weightofrandomcolor_3) (- 1.0 _weightofrandomcolor_3)) :!class /Script/Engine.MaterialInstanceDynamic)
  (Transformation|SetRelativeTransform (Variables|Default|GetStaticMesh) (Math|Transform|MakeTransform "0, 0, 0" (Math|Rotator|MakeRotator 0.0 0.0 (* (Math|Random|RandomFloat) 3.6e+02)) (Math|Vector|MakeVector 1.0 1.0 (+ (* (Math|Random|RandomFloat) _weightofrandomscale) (- 1.0 _weightofrandomscale)))) false true))