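; BP_Stone is a ground prop stone that randomizes its look so that placed copies vary.
; The construction script randomly mirrors the SMStone mesh on X and Y with ±1 scale and varies its height.
; It then randomizes the RedSubstitute, GreenSubstitute and BlueSubstitute vector parameters on the mesh's materials within narrow ranges.
; The event graph holds only disabled placeholder events, so all logic runs at construction.
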(event EventBeginPlay)

(event Collision|EventActorBeginOverlap
  (params (OtherActor :type Actor%20Object%20Reference)))

(event EventTick
  (params (DeltaSeconds :type Float%20%28single-precision%29)))

(fn ConstructionScript
  (bind _returnvalue (Math|Random|RandomFloatinRange 0.1 0.15))
  (bind _sm_stone (Variables|Default|GetSM_Stone))
  (Transformation|SetRelativeScale3D _sm_stone (Math|Vector|MakeVector (Math|Conversions|ToFloat(Integer) (- (* (Math|Conversions|ToInteger(Boolean) (Math|Random|RandomBool)) 2) 1)) (Math|Conversions|ToFloat(Integer) (- (* (Math|Conversions|ToInteger(Boolean) (Math|Random|RandomBool)) 2) 1)) (Math|Random|RandomFloatinRange 0.5 1.5)))
  (Rendering|Material|SetVectorParameterValueonMaterials _sm_stone "RedSubstitute" (Math|Vector|MakeVector (Math|Random|RandomFloatinRange 0.0 0.005) (Math|Random|RandomFloatinRange 0.01 0.2) 0.0))
  (Rendering|Material|SetVectorParameterValueonMaterials _sm_stone "GreenSubstitute" (Math|Vector|MakeVector (Math|Random|RandomFloatinRange 0.1 0.12) (Math|Random|RandomFloatinRange 0.1 0.12) (Math|Random|RandomFloatinRange 0.12 0.15)))
  (Rendering|Material|SetVectorParameterValueonMaterials _sm_stone "BlueSubstitute" (Math|Vector|MakeVector _returnvalue _returnvalue _returnvalue)))