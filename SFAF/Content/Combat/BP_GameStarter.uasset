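; Combat bootstrapper that spawns the player and AI teams, then starts combat.
; It waits in stages for the grid, combat system and add/remove-unit action, polling for each actor and binding to its ready event.
; Team size follows saved round history, capped by grid size, and win/loss streaks adjust the difficulty for the AI's second spawn pass.
; It also saves, loads and erases round results in the CommonSave slot.
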(event Custom|Event_GridIsReady
  ;[0.01 0.01 0.01] Actions also can take a while to be ready to use
  (Variables|Default|SetPositions (Default|GetAllGridPositions (Variables|Default|GetGrid)))
  (bind _returnvalue (Actor|GetActorOfClass "/Game/Combat/BP_CombatSystem.BP_CombatSystem_C" :!label _label))
  (bind _output_get (Variables|Default|SetCombatSystem _returnvalue))
  (Utilities|IsValid _output_get
    (:Is%20Valid
      (EventDispatchers|BindEventtoOnCombatFinishing _output_get (EventDispatchers|CreateEvent :!event FinishedGameRegistry))
      (if (Default|IsCombatSystemReady (Variables|Default|GetCombatSystem))
        (CallFunction|EventCombatSystemIsReady)
        (else
          (EventDispatchers|AssignOnCombatSystemReady (Variables|Default|GetCombatSystem) (delegate Custom|Event_CombatSystemIsReady)))))
    (:Is%20Not%20Valid
      (Utilities|FlowControl|Delay 0.2)
      (goto _label))))

(event Custom|Event_ToStartCombat
  (bind _combatsystem (Variables|Default|GetCombatSystem))
  (bind (_canstartcombat _enoughunits _enoughteams _notincombat) (Default|CanStartCombat _combatsystem))
  ;[0.01 0.01 0.01] Only then it is ready for combat.
  (if _canstartcombat
    (Default|StartCombat (Variables|Default|GetCombatSystem))
    ;[0.01 0 0.01] Faster way to solve a bug
    (Utilities|FlowControl|Delay 0.1)
    (bind _returnvalue (Actor|GetActorOfClass "/Game/TopDown/Blueprints/BP_AITacticalController.BP_AITacticalController_C"))
    (Default|SelectLastTile _returnvalue)
    ;[0.01 0 0.01] It can happen that combat not start
    (Utilities|FlowControl|Delay 0.2)
    (if (not (Default|GetIsinCombat (Variables|Default|GetCombatSystem)))
      (Default|StartCombat (Variables|Default|GetCombatSystem)))
    (else
      (Development|PrintString (Utilities|String|Append "Cannot Start Combat" " Enough Units: " (Utilities|String|ToString(Boolean) _enoughunits) " Enought Teams: " (Utilities|String|ToString(Boolean) _enoughteams) " Already In Combat: " (Utilities|String|ToString(Boolean) _notincombat))))))

(event Custom|Event_InitialSettings
  ;[0.01 0.01 0.01] Grid Can Take Time to Spawn. After finished to spawn all hexagons, need to start second fase of this BP.
  (Variables|Default|SetNextPositionToSpawn 0)
  (CallFunction|LoadSingleGame)
  (Utilities|FlowControl|Delay 0.1 :!label _label)
  (bind _returnvalue (Actor|GetActorOfClass "/Game/Ground/Terrain/BP_Grid.BP_Grid_C"))
  (bind _output_get (Variables|Default|SetGrid _returnvalue))
  (Utilities|IsValid _output_get
    (:Is%20Valid
      (if (Default|IsGridReady (Variables|Default|GetGrid))
        (CallFunction|EventGridIsReady)
        (else
          (EventDispatchers|AssignOnGridUpdatedFinished (Variables|Default|GetGrid) (delegate Custom|Event_GridIsReady)))))
    (:Is%20Not%20Valid
      (goto _label))))

(event Custom|Event_CombatSystemIsReady
  ;[0.01 0.01 0.01] It can take a while to Combat System get ready.
  (bind _returnvalue (Actor|GetActorOfClass "/Game/Characters/Actions/Combat/BP_ActionAddRemoveUnitFromCombat.BP_ActionAddRemoveUnitFromCombat_C" :!label _label))
  (bind _output_get (Variables|Default|SetAddRemoveUnit _returnvalue))
  (Utilities|IsValid _output_get
    (:Is%20Valid
      (if (Class|ActionBase|GetReady (Variables|Default|GetAddRemoveUnit))
        (CallFunction|EventSpawnTeam)
        (else
          (EventDispatchers|BindEventtoReadytoUse (Variables|Default|GetAddRemoveUnit) (EventDispatchers|CreateEvent :!event Custom|Event_SpawnTeam)))))
    (:Is%20Not%20Valid
      (Utilities|FlowControl|Delay 0.2)
      (goto _label))))

(event Custom|Event_StartPlaying
  (Variables|Default|SetbHasStarted true)
  (Utilities|FlowControl|Delay 0.6)
  (bind _returnvalue (SaveGame|DoesSaveGameExist "CommonSave"))
  (if _returnvalue
    _
    (else
      (CallFunction|SaveSingleGame)))
  (CallFunction|EventInitialSettings))

(event EventBeginPlay
  (Variables|Default|SetbHasStarted true)
  (Utilities|FlowControl|Delay 0.6)
  (bind _returnvalue (SaveGame|DoesSaveGameExist "CommonSave"))
  (if _returnvalue
    _
    (else
      (CallFunction|SaveSingleGame)))
  (CallFunction|EventInitialSettings))

(event Custom|Event_SpawnTeam
  (Default|SetIsAddingUnit (Variables|Default|GetAddRemoveUnit) true)
  (if (Utilities|Map|IsEmpty (Variables|Default|GetVictories))
    _
    (else
      (bind _values (Utilities|Map|Values (Variables|Default|GetVictories)))
      (Variables|SpawnTeam|SetQuantityOfInteractionsToLoop _values)))
  ;[0 0.1042 0] The Quantity of units is according with victories, but I did an adjust on end of the loop to give the AI Team a little more than the player, if necessary
  (Utilities|Array|Add (Variables|SpawnTeam|GetQuantityOfInteractionsToLoop) true)
  ;[0.1 0 0] Limit the quantity of units to spawn per team.
  (Variables|SpawnTeam|SetQuantityOfPositionsToUse (/ (Utilities|Array|Length (Variables|Default|GetPositions)) (* (Variables|SpawnTeam|GetSpaceBetweenUnit) (Variables|SpawnTeam|GetDifficultSetting))))
  (bind _array_element (Utilities|Array|ForEachLoopwithBreak (Variables|SpawnTeam|GetQuantityOfInteractionsToLoop) :!label _label)
    (:LoopBody
      (CallFunction|SpawnUnit _array_element)
      ;[0.05729 0.05729 0.05729] I need to be careful and not try to spawn more units than the grid can resist.
      (bind _output_get (Variables|SpawnTeam|SetCountSpawnedUnit (+ (Variables|SpawnTeam|GetCountSpawnedUnit) 1)))
      (if (>= _output_get (/ (Variables|SpawnTeam|GetQuantityOfPositionsToUse) 2))
        (goto _label Break)))
    (:Completed
      (Utilities|FlowControl|FlipFlop
        (:A
          (Utilities|FlowControl|Delay 0.2)
          (Variables|SpawnTeam|SetAITeam true)
          (Variables|SpawnTeam|SetUnitTypeTag "(TagName=\"Unit.Type.Harvester\")")
          (Variables|SpawnTeam|SetDifficultRegulator (- (+ (Math|Integer|%(Integer) (Variables|SpawnTeam|GetCountConsecutiveVictories) (Variables|SpawnTeam|GetDifficultChanger)) (Variables|SpawnTeam|GetDifficultRegulator)) (Math|Integer|%(Integer) (Variables|SpawnTeam|GetCountConsecutiveDefeats) (Variables|SpawnTeam|GetDifficultChanger))))
          ;[0 0.01 0.01] Difficult settings according with victories/defeates consecutives
          (Variables|SpawnTeam|SetDifficultSetting (+ (Variables|SpawnTeam|GetDifficultSetting) (Variables|SpawnTeam|GetDifficultRegulator)))
          (goto _label))
        (:B
          (Default|SetIsAddingUnit (Variables|Default|GetAddRemoveUnit) false)
          (CallFunction|EventtoStartCombat))))))

(fn ConstructionScript)

(fn FinishedGameRegistry
  (params (WinnerTeam :type Byte))
  (bind _output_get (Variables|Default|SetRounds (+ (Variables|Default|GetRounds) 1)))
  (Utilities|Map|Add (Variables|Default|GetVictories) _output_get (== WinnerTeam (Variables|Default|GetPlayerTeam)))
  (CallFunction|SaveSingleGame))

(fn SaveSingleGame
  (bind _returnvalue (SaveGame|CreateSaveGameObject "/Game/TopDown/Blueprints/BP_CommonSaveGame.BP_CommonSaveGame_C"))
  (bind _output_get (Variables|Default|SetSaveGame _returnvalue))
  (Default|SetVariables _output_get (Variables|Default|GetRounds) (Variables|Default|GetVictories))
  (bind _returnvalue_2 (SaveGame|SaveGametoSlot _output_get "CommonSave")))

(fn LoadSingleGame
  (bind _returnvalue (SaveGame|LoadGamefromSlot "CommonSave"))
  (bind _asbp_common_save_game (Utilities|Casting|CastToBP_CommonSaveGame _returnvalue)
    (:then
      (bind _output_get (Variables|Default|SetSaveGame _asbp_common_save_game))
      (bind _output_get_2 (Variables|Default|SetRounds (.PlayedRounds (Default|GetVariables _output_get))))
      (bind _output_get_3 (Variables|Default|SetVictories (.PlayerVictories (Default|GetVariables _output_get)))))
    (:CastFailed
      (Development|PrintString "Error on GameStarter: SaveGame Cast Failed."))))

(fn EraseSaveGame
  (bind _returnvalue (SaveGame|DeleteGameinSlot "CommonSave"))
  (Variables|Default|SetRounds 0)
  (Utilities|Map|Clear (Variables|Default|GetVictories))
  (Development|PrintString (Utilities|String|Append "File deleted? " (Utilities|String|ToString(Boolean) _returnvalue))))

(fn HasStarted
  (return (Variables|Default|GetbHasStarted)))

(fn SpawnUnit
  (params (bVictory :type Boolean))
  (Utilities|FlowControl|Sequence
    (:then_0
      (Default|SetUnitTypeTag (Variables|Default|GetAddRemoveUnit) (Variables|SpawnTeam|GetUnitTypeTag))
      ;[0 0.06771 0] Choosing Team, in the simple way.
      (Default|SetTeamNumber (Variables|Default|GetAddRemoveUnit) (select (Variables|SpawnTeam|GetAITeam) 2 1))
      (Default|SetUseAI (Variables|Default|GetAddRemoveUnit) (Variables|SpawnTeam|GetAITeam))
      (Default|AddUnit :self (Variables|Default|GetAddRemoveUnit))
      (Variables|Default|SetNextPositionToSpawn (+ (Variables|Default|GetNextPositionToSpawn) (Variables|SpawnTeam|GetSpaceBetweenUnit)))
      ;[0 0 0.1354] I could do more complex. But looks satisfatory: Half of units is a specific type.
      (if (not (== (Variables|SpawnTeam|GetUnitTypeTag) "(TagName=\"Unit.Type.Anthill\")"))
        (if (== (Variables|SpawnTeam|GetUnitTypeTag) "(TagName=\"Unit.Type.BulletAnt\")")
          (Variables|SpawnTeam|SetUnitTypeTag "(TagName=\"Unit.Type.Wasp\")")
          (elif (== (Variables|SpawnTeam|GetUnitTypeTag) "(TagName=\"Unit.Type.Wasp\")")
            (Variables|SpawnTeam|SetUnitTypeTag "(TagName=\"Unit.Type.BulletAnt\")")
            (elif (== (Variables|SpawnTeam|GetUnitTypeTag) "(TagName=\"Unit.Type.Harvester\")")
              (Variables|SpawnTeam|SetUnitTypeTag "(TagName=\"Unit.Type.Truck\")")
              (elif (== (Variables|SpawnTeam|GetUnitTypeTag) "(TagName=\"Unit.Type.Truck\")")
                (Variables|SpawnTeam|SetUnitTypeTag "(TagName=\"Unit.Type.Harvester\")")))))))
    (:then_1
      (if (not (Variables|SpawnTeam|GetAITeam))
        (if bVictory
          (Variables|SpawnTeam|SetCountConsecutiveDefeats 0)
          (Variables|SpawnTeam|SetCountConsecutiveVictories (+ (Variables|SpawnTeam|GetCountConsecutiveVictories) 1))
          (else
            (Variables|SpawnTeam|SetCountConsecutiveVictories 0)
            (Variables|SpawnTeam|SetCountConsecutiveDefeats (+ (Variables|SpawnTeam|GetCountConsecutiveDefeats) 1))))))))