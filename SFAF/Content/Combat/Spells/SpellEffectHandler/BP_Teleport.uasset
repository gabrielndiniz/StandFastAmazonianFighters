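; Spell effect handler for the Teleport spell, which moves the combatant on the caster's grid tile to a target tile.
; If the target tile exists and is unoccupied, it force-moves the unit through BP_CombatSystem and writes back the origin tile's data.
; A post-teleport event waits briefly, then clears the cast-spell state and retriggers the click on player 0's tactical grid controller, assuming single-player.
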(event Custom|Event_PostTeleport
  (Utilities|FlowControl|Delay 0.1)
  (bind _asbp_tactical_grid_controller (Utilities|Casting|CastToBP_TacticalGridController (Game|GetPlayerController 0))
    (:then
      (Default|SetCastSpell (Default|GetActionManager _asbp_tactical_grid_controller) false)
      (Default|EventRetriggerClick _asbp_tactical_grid_controller))
    (:CastFailed
      (Development|PrintString "Error: Not found PlayerController"))))

(fn ConstructionScript
  (|CallParentFunction))

(fn SpellEffect
  (bind _targetposition (Variables|Default|GetTargetPosition))
  (bind _grid (Variables|Default|GetGrid))
  (bind (_success _tiledata) (Default|GetTileData _grid _targetposition))
  (|CallParentFunction)
  (if _success
    (bind _returnvalue (Actor|GetActorOfClass "/Game/Combat/BP_CombatSystem.BP_CombatSystem_C"))
    (Utilities|IsValid (.OccupyingUnit (Utilities|Struct|BreakGridTileOccupancy (.Occupancy (Utilities|Struct|BreakGridTileStaticData _tiledata))))
      (:Is%20Not%20Valid
        (bind _asbp_combatant_base (Utilities|Casting|CastToBP_Combatant_Base (.OccupyingUnit (Utilities|Struct|BreakGridTileOccupancy (.Occupancy (Utilities|Struct|BreakGridTileStaticData (.TileData (Default|GetTileData (Variables|Default|GetGrid) (Variables|Default|GetUnitPosition)))))))))
        (bind _output_get (LocalVariables|SetTeleportUnit _asbp_combatant_base))
        (Utilities|IsValid _output_get
          (:Is%20Valid
            (Default|SetUnitPositiononGrid _returnvalue (LocalVariables|GetTeleportUnit) (Variables|Default|GetTargetPosition) false true true)
            (CallFunction|EventPostTeleport)
            (Default|AddTileData (Variables|Default|GetGrid) (Variables|Default|GetUnitPosition) (.TileData (Default|GetTileData (Variables|Default|GetGrid) (Variables|Default|GetUnitPosition)))))
          (:Is%20Not%20Valid
            (Development|PrintString "Error: Not found Unit")))))))