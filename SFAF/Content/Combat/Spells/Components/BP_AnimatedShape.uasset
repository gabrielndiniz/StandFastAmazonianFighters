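; BP_AnimatedShape is a spell component actor that animates a shape from an origin transform to a target, then destroys itself after a short delay.
; SetTransforms stores both transforms and a Position, faces the target and starts a timeline whose play rate scales inversely with distance.
; The timeline interpolates the transform with height, rotation and scale modifiers.
; On finish it snaps to the target, fires OnShapeAnimationCompleted and calls the empty AnimationComplete hook.
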(event Custom|StartAnimation
  (bind _targettransform (Variables|Default|GetTargetTransform))
  (Components|Timeline|SetPlayRate (Variables|Default|GetPlayAnimationTimeline) (/ (Variables|Default|GetSpeed) (/ (Math|Float|Clamp(Float) (Math|Vector|Distance(Vector) (.location (Variables|Default|GetOriginTransform)) (.location (Variables|Default|GetTargetTransform))) 0.5 999999.0) (Variables|Default|GetSpeedAdjust))))
  (bind (_direction _transformalpha _heightoffset) (Timeline|PlayAnimationTimeline PlayFromStart)
    (:Update
      (Variables|Default|SetLocationModifier (Math|Vector|MakeVector 0.0 0.0 (* (Variables|Default|GetMaxHeight) _heightoffset)))
      (Transformation|SetActorTransform (Math|Transform|MakeTransform (+ (.location (Math|Transform|Lerp(Transform) (Variables|Default|GetOriginTransform) (Variables|Default|GetTargetTransform) _transformalpha)) (Variables|Default|GetLocationModifier)) (Math|Rotator|CombineRotators (.rotation (Math|Transform|Lerp(Transform) (Variables|Default|GetOriginTransform) (Variables|Default|GetTargetTransform) _transformalpha)) (Variables|Default|GetRotatorModifier)) (* (.scale (Math|Transform|Lerp(Transform) (Variables|Default|GetOriginTransform) (Variables|Default|GetTargetTransform) _transformalpha)) (Variables|Default|GetScaleModifier)))))
    (:Finished
      (Transformation|SetActorTransform (Math|Transform|MakeTransform (.location _targettransform) (.rotation _targettransform) (* (.scale _targettransform) (Variables|Default|GetScaleModifier))))
      (Default|CallOnShapeAnimationCompleted self)
      (CallFunction|AnimationComplete)
      (Utilities|FlowControl|Delay 2.0)
      (Actor|DestroyActor))))

(fn ConstructionScript)

(fn SetTransforms
  (params (OriginTransform :type Transform) (TargetTransform :type Transform) (Position :type Int%20Point%20Structure))
  (bind _output_get (Variables|Default|SetOriginTransform OriginTransform))
  (bind _output_get_2 (Variables|Default|SetTargetTransform TargetTransform))
  (Transformation|SetActorRotation (Math|Rotator|FindLookatRotation (.location _output_get) (.location _output_get_2)))
  (Variables|Default|SetPosition Position)
  (CallFunction|StartAnimation))

(fn AnimationComplete)

(fn GetTargetPosition
  (return (Variables|Default|GetPosition)))