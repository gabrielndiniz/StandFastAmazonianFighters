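; Grid spell animation actor that starts hidden at zero scale and plays a spell's visual on its target tiles.
; It starts on its own or, via SetBasics, waits for another cast's completion to chain after it.
; Playing spawns an animated shape per target position; each finished shape broadcasts a tile hit.
; Once all targets finish, it broadcasts completion and destroys itself after a short delay.
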(event Custom|Event_PlaySpellAnimation
  (Transformation|SetActorScale3D "1.000000,1.000000,1.000000")
  (for _array_element (Variables|Default|GetTargetPositions)
    (Variables|Default|SetCurrentTargetPosition _array_element)
    (bind _returnvalue (Game|SpawnActorfromClass (Variables|Default|GetAnimatedShapeClass) (Math|Transform|MakeTransform (.worldlocation (.TileData (Default|GetTileData (Variables|Default|GetGrid)))) "0, 0, 0" "1.000000,1.000000,1.000000") "AlwaysSpawn" "SelectDefaultAtRuntime" 0 0))
    (EventDispatchers|BindEventtoOnShapeAnimationCompleted _returnvalue (delegate Custom|OnShapeAnimationCompleted))
    (Default|SetTransforms _returnvalue (Math|Transform|MakeTransform (.worldlocation (.TileData (Default|GetTileData (Variables|Default|GetGrid)))) "0, 0, 0" "1.000000,1.000000,1.000000") (Math|Transform|MakeTransform (.worldlocation (.TileData (Default|GetTileData (Variables|Default|GetGrid)))) "0, 0, 0" "1.000000,1.000000,1.000000") (Variables|Default|GetCurrentTargetPosition))))

(event Custom|Event_ForcePlay
  (bind _returnvalue (Transformation|GetActorLocation))
  (bind _returnvalue_2 (Game|SpawnActorfromClass (Variables|Default|GetAnimatedShapeClass) (Math|Transform|MakeTransform (Transformation|GetActorLocation) "0, 0, 0" "10.000000,10.000000,10.000000") "AlwaysSpawn" "SelectDefaultAtRuntime" 0 0))
  (Default|SetTransforms _returnvalue_2 (Math|Transform|MakeTransform _returnvalue "0, 0, 0" "10.000000,10.000000,10.000000") (Math|Transform|MakeTransform _returnvalue "0, 0, 0" "10.000000,10.000000,10.000000")))

(event Custom|CompletedSpellAnimation
  (Default|CallOnSpellAnimationCompleted self)
  (Utilities|FlowControl|Delay 0.2)
  (Actor|DestroyActor))

(event Custom|OnShapeAnimationCompleted
  (params (AnimatedShape :type BP%20Animated%20Shape%20Object%20Reference))
  (bind _position (Default|GetTargetPosition AnimatedShape))
  (bind _targetpositions (Variables|Default|GetTargetPositions))
  (Utilities|Array|AddUnique (Variables|Default|GetAnimated%20Shapes) AnimatedShape)
  (Default|CallOnSpellHitTile self _position)
  (Utilities|Array|RemoveItem _targetpositions _position)
  (if (== (Utilities|Array|Length _targetpositions) 0)
    (CallFunction|CompletedSpellAnimation)))

(event EventBeginPlay
  (Transformation|SetActorScale3D "0, 0, 0")
  (Utilities|FlowControl|Delay 0.2)
  (if (Variables|Default|GetbStart)
    (CallFunction|EventPlaySpellAnimation)))

(fn ConstructionScript)

(fn SetBasics
  (params (Grid :type BP%20Grid%20Object%20Reference) (OriginPosition :type Int%20Point%20Structure) (TargetPosition :type Int%20Point%20Structure) (bStart :type Boolean) (OriginCast :type BP%20Spell%20Animation%20Object%20Reference))
  (Variables|Default|SetGrid Grid)
  (Variables|Default|SetOriginPosition OriginPosition)
  (Utilities|Array|Add (Variables|Default|GetTargetPositions) TargetPosition)
  (bind _output_get (Variables|Default|SetbStart bStart))
  (if (not _output_get)
    (Utilities|IsValid OriginCast
      (:Is%20Valid
        (EventDispatchers|BindEventtoOnSpellAnimationCompleted OriginCast (EventDispatchers|CreateEvent :!event OnFinishedRangeCast)))
      (:Is%20Not%20Valid
        (CallFunction|OnFinishedRangeCast)))))

(fn OnFinishedRangeCast
  (params (SpellAnimation :type BP%20Spell%20Animation%20Object%20Reference))
  (CallFunction|EventPlaySpellAnimation))