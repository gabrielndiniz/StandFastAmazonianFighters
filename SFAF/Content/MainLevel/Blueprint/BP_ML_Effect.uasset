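; BP_ML_Effect is a main-level effect actor that plays a timed smoke screen on every ally, followed by a scale change.
; On BeginPlay it caches all BP_Ally actors, then after a short delay spawns a BP_SmokeScreen at each one's location and triggers its EventForcePlay.
; After a second delay it sets the scale of each cached ally, so the change follows the smoke.
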(event EventBeginPlay
  (bind _outactors (Actor|GetAllActorsOfClass "/Game/Characters/Allies/BP_Ally.BP_Ally_C"))
  (Variables|Default|SetAllies _outactors)
  (Utilities|FlowControl|Delay 1.0)
  (for _array_element (Variables|Default|GetAllies)
    (bind _returnvalue (Game|SpawnActorfromClass "/Game/Combat/Spells/SpellsAnimations/BP_SmokeScreen.BP_SmokeScreen_C" (Math|Transform|MakeTransform (Math|Vector|MakeVector (.x (Transformation|GetActorLocation _array_element)) (.y (Transformation|GetActorLocation _array_element)) (+ (.z (Transformation|GetActorLocation _array_element)) 0.0)) "0, 0, 0" "1.000000,1.000000,1.000000") "Undefined" "OverrideRootScale" 0 0))
    (Default|EventForcePlay _returnvalue))
  (Utilities|FlowControl|Delay 1.0)
  (for _array_element_2 (Variables|Default|GetAllies)
    (Transformation|SetActorScale3D _array_element_2 (Variables|Default|GetNew%20Scale%203D))))

(fn ConstructionScript)